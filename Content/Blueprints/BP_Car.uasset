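; Car actor that drives along a spline in one of two lanes, with a configurable mesh, speed and start position.
; Each Tick it adds Speed to its distance, without delta-time scaling, and snaps to a point offset sideways from the spline.
; The Right flag selects forward travel or mirrored travel from the spline's end, with opposite offset and 180-degree rotation.
; It destroys itself outside the spline's length or after 20 real-time seconds.
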(event `self.ReceiveBeginPlay`
  (bind (_seconds _partialseconds) (`GameplayStatics.GetAccurateRealTime`))
  (set `self.StartTime` (+ (`KismetMathLibrary.Conv_IntToDouble` _seconds) _partialseconds))
  (`StaticMeshComponent.SetStaticMesh` (`self.StaticMesh`) (`self.Mesh`)))

(event `self.ReceiveTick`
  (params (DeltaSeconds :type "Float (single-precision)"))
  (bind (_seconds _partialseconds) (`GameplayStatics.GetAccurateRealTime`))
  (bind _right (`self.Right`))
  (bind _spline (`self.spline`))
  (bind _spline_2 (`self.spline`))
  (bind _returnvalue (`SplineComponent.GetSplineLength` _spline))
  (bind _returnvalue_2 (+ (`self.LocationOnSpline`) (`self.startPosition`)))
  (bind _returnvalue_3 (+ (`self.LocationOnSpline`) (`self.startPosition`)))
  (bind _returnvalue_4 (- _returnvalue (+ (`self.LocationOnSpline`) (`self.startPosition`))))
  (set `self.LocationOnSpline` (+ (`self.LocationOnSpline`) (`self.Speed`)))
  (if (< (- (+ (`KismetMathLibrary.Conv_IntToDouble` _seconds) _partialseconds) (`self.StartTime`)) 20.0)
    (if (and (> _returnvalue_2 0.0) (< _returnvalue_2 _returnvalue))
      (`SceneComponent.K2_SetWorldLocationAndRotation` (`self.DefaultSceneRoot`) (`KismetMathLibrary.SelectVector` (`/Game/Blueprints/EditorUtility/BFL_SplineCorrector.GetRightPointAtDistanceAtDistanceAlongSpline` _spline_2 _returnvalue_3 300.0 "World") (`/Game/Blueprints/EditorUtility/BFL_SplineCorrector.GetRightPointAtDistanceAtDistanceAlongSpline` _spline _returnvalue_4 -300.0 "World") _right) (`KismetMathLibrary.SelectRotator` (`SplineComponent.GetRotationAtDistanceAlongSpline` _spline_2 _returnvalue_3 "World") (`KismetMathLibrary.ComposeRotators` (`SplineComponent.GetRotationAtDistanceAlongSpline` _spline _returnvalue_4 "World") (struct :`Yaw` 180.0)) _right) false false)
      (else
        (`self.K2_DestroyActor`)))
    (else
      (`self.K2_DestroyActor`))))

(fn `UserConstructionScript`)