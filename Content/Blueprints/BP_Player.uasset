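; VR player for the Brussels Volocopter demo, handling start screen, hands and tutorial.
; Grip and trigger inputs animate mirrored hand meshes and drive grabbing and finger collision checks.
; Tick runs a voiced tutorial state machine with blinking controllers, repeat timers and checks for fist, camera and flight stick.
; Completing or skipping it fades out the tutorial sphere and starts the Volocopter; screen transitions use a Material Parameter Collection.
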(event `Key|MotionController_Left_Grip1` :consume false
  (params (Key :type "Key Structure"))
  (:`Pressed`
    (if true :!label _label
      (if (`self.IsInStartScreen`) :!label _label_2
        (`self.ForceHandsVisible`)
        (`KismetSystemLibrary.PrintString` "End Startscreen" true true (struct :`R` 1.0 :`G` 0.234878 :`A` 1.0))
        (`/Game/Blueprints/BP_startScreen.StartTheGame` (cast `/Game/Blueprints/BP_startScreen` (`ChildActorComponent.ChildActor` (`self.StartScreen`)) :!pure true))
        (`self.PPTransition` 4.0 3.0 (struct :`R` 0.807292 :`G` 0.807292 :`B` 0.807292 :`A` 1.0))
        (`KismetSystemLibrary.Delay` 2.0)
        (`SceneComponent.SetVisibility` (`self.StartScreen`) true true)
        (set `self.IsInStartScreen` false)
        (`/Game/Blueprints/BP_DroneportGameMode.StartGame` (cast `/Game/Blueprints/BP_DroneportGameMode` (`GameplayStatics.GetGameMode`) :!pure true))
        (`self.RecalibrateHmd`)
        (set `self.TutorialActiveBool` true)))))

(event `Key|MotionController_Right_Grip1` :consume false
  (params (Key :type "Key Structure"))
  (:`Pressed`
    (goto _label)))

(event `Key|MotionController_Left_Trigger` :consume false
  (params (Key :type "Key Structure"))
  (:`Pressed`
    (goto _label)))

(event `Key|MotionController_Right_Trigger` :consume false
  (params (Key :type "Key Structure"))
  (:`Pressed`
    (goto _label)))

(event `Key|MotionController_Left_FaceButton1`
  (params (Key :type "Key Structure"))
  (:`Pressed`
    (goto _label)))

(event `Key|MotionController_Right_FaceButton1`
  (params (Key :type "Key Structure"))
  (:`Pressed`
    (goto _label)))

(event `Key|MotionController_Left_FaceButton2`
  (params (Key :type "Key Structure"))
  (:`Pressed`
    (goto _label)))

(event `Key|MotionController_Right_FaceButton2`
  (params (Key :type "Key Structure"))
  (:`Pressed`
    (goto _label)))

(event `Key|MotionController_Left_FaceButton3`
  (params (Key :type "Key Structure"))
  (:`Pressed`
    (goto _label)))

(event `Key|MotionController_Right_FaceButton3`
  (params (Key :type "Key Structure"))
  (:`Pressed`
    (goto _label)))

(event `Key|MotionController_Left_FaceButton4`
  (params (Key :type "Key Structure"))
  (:`Pressed`
    (goto _label)))

(event `Key|MotionController_Right_FaceButton4`
  (params (Key :type "Key Structure"))
  (:`Pressed`
    (goto _label)))

(event `Key|BackSpace`
  (params (Key :type "Key Structure"))
  (:`Pressed`
    (goto _label_2)))

(event `Key|MotionController_Right_Trigger`
  (params (Key :type "Key Structure"))
  (bind __prighthandmesh (`self._pRightHandMesh`))
  ;[1 1 1] Hand Controls
  (:`Pressed`
    (`self.SetAnimState` "INDEX" "CLOSED" __prighthandmesh)
    (`self.SetHandState` "RIGHT_INDEX")
    (`self.CheckForFingerCollision` true)
    (set `self._MotionControllerRTriggerHold` true))
  (:`Released`
    (`self.SetAnimState` "INDEX" "OPEN" __prighthandmesh)
    (`self.ClearHandState` "RIGHT_INDEX")
    (`self.CheckForFingerCollision` true)
    (set `self._MotionControllerRTriggerHold` false)))

(event `Key|MotionController_Right_Grip1`
  (params (Key :type "Key Structure"))
  (bind __prighthandmesh (`self._pRightHandMesh`))
  ;[1 1 1] Hand Controls
  (:`Pressed`
    (`self.SetAnimState` "CORE" "CLOSED" __prighthandmesh)
    (`self.SetHandState` "RIGHT_CORE")
    (`self.CheckForGrabCollision` (`self._pGrabColliderRight`) "RIGHT_CORE")
    (`self.CheckForFingerCollision` true)
    (set `self._MotionControllerRGripHold` true))
  (:`Released`
    (`self.SetAnimState` "CORE" "OPEN" __prighthandmesh)
    (`self.ClearHandState` "RIGHT_CORE")
    (`self.TryRelease` (`self._pRightHandMesh`) (`self._pGrabColliderRight`))
    (`self.CheckForFingerCollision` true)
    (set `self._MotionControllerRGripHold` false)))

(event `Key|MotionController_Left_Trigger`
  (params (Key :type "Key Structure"))
  (bind __plefthandmesh (`self._pLeftHandMesh`))
  ;[1 1 1] Hand Controls
  (:`Pressed`
    (`self.SetAnimState` "INDEX" "CLOSED" __plefthandmesh)
    (`self.SetHandState` "LEFT_INDEX")
    (`self.CheckForFingerCollision` false)
    (set `self._MotionControllerLTriggerHold` true))
  (:`Released`
    (`self.SetAnimState` "INDEX" "OPEN" __plefthandmesh)
    (`self.ClearHandState` "LEFT_INDEX")
    (`self.CheckForFingerCollision` false)
    (set `self._MotionControllerLTriggerHold` false)))

(event `Key|MotionController_Left_Grip1`
  (params (Key :type "Key Structure"))
  (bind __plefthandmesh (`self._pLeftHandMesh`))
  ;[1 1 1] Hand Controls
  (:`Pressed`
    (`self.SetAnimState` "CORE" "CLOSED" __plefthandmesh)
    (`self.SetHandState` "LEFT_CORE")
    (`self.CheckForGrabCollision` (`self._pGrabColliderLeft`) "LEFT_CORE")
    (`self.CheckForFingerCollision` false)
    (set `self._MotionControllerLGripHold` true))
  (:`Released`
    (`self.SetAnimState` "CORE" "OPEN" __plefthandmesh)
    (`self.ClearHandState` "LEFT_CORE")
    (`self.TryRelease` (`self._pLeftHandMesh`) (`self._pGrabColliderLeft`))
    (`self.CheckForFingerCollision` false)
    (set `self._MotionControllerLGripHold` false)))

(event `FadeOutStartSphere`
  (bind (_direction _tutorialspace) (`Timeline|StartSphere` :!via `PlayFromStart` :!label _label_3)
    (:`Update`
      (`MaterialInstanceDynamic.SetScalarParameterValue` (`self.TutorialMat`) "Opacity" _tutorialspace))))

(event `FadeInStartSphere`
  (goto _label_3 :!via `ReverseFromEnd`))

(event `self._pGrabColliderLeft.OnComponentBeginOverlap`
  (params (OverlappedComponent :type "PrimitiveComponent Object Reference") (OtherActor :type "Actor Object Reference") (OtherComp :type "PrimitiveComponent Object Reference") (OtherBodyIndex :type Integer) (bFromSweep :type Boolean) (SweepResult :type "HitResult Structure (by ref)"))
  ;[1 1 1] Grabbing
  (`self.TryGrab` OtherActor (`self._pLeftHandMesh`) (`self._pGrabColliderLeft`) (`self._pLeftGrabOffset`)))

(event `self._pGrabColliderRight.OnComponentBeginOverlap`
  (params (OverlappedComponent :type "PrimitiveComponent Object Reference") (OtherActor :type "Actor Object Reference") (OtherComp :type "PrimitiveComponent Object Reference") (OtherBodyIndex :type Integer) (bFromSweep :type Boolean) (SweepResult :type "HitResult Structure (by ref)"))
  ;[1 1 1] Grabbing
  (`self.TryGrab` OtherActor (`self._pRightHandMesh`) (`self._pGrabColliderRight`) (`self._pRightGrabOffset`)))

(event `Key|SpaceBar`
  (params (Key :type "Key Structure"))
  (:`Pressed`
    (bind _returnvalue (`GameplayStatics.GetActorOfClass` "/Game/Blueprints/BP_VolocopterPath.BP_VolocopterPath_C"))
    (`/Engine/EditorBlueprintResources/StandardMacros.IsValid` _returnvalue
      (:`Is Valid`
        (`/Game/Blueprints/BP_VolocopterPath.Teleport` _returnvalue 10000.0)))))

(event `self.ReceiveBeginPlay`
  (`self.SetControllerMaterials`)
  (`self.Set Material`))

(event `Reset Tutorial`
  (goto _label_4 :!via `Reset`))

(event `self.HandleGameReset`
  (set `self.IsInStartScreen` true)
  (`AudioComponent.Stop` (`self._AudioPlayer`))
  (`self.Reset Tutorial`)
  (`self.FadeInStartSphere`)
  (`SceneComponent.SetVisibility` (`self.TutorialSpace`) true false)
  (bind _returnvalue (`GameplayStatics.GetActorOfClass` "/Game/Blueprints/BP_EndBox.BP_EndBox_C"))
  (`/Game/Blueprints/BP_EndBox.Reset Endgame` _returnvalue))

(event `Set Material`
  (bind _returnvalue (`PrimitiveComponent.CreateDynamicMaterialInstance` (`self.TutorialSpace`) 0 "/Game/artAssets/tex/M_Fade_startSphere.M_Fade_startSphere" "None"))
  (bind _output_get (set `self.TutorialMat` _returnvalue))
  (`PrimitiveComponent.SetMaterial` (`self.TutorialSpace`) 0 _output_get)
  (`KismetSystemLibrary.PrintString` "Mat Set" true true (struct :`R` 1.0 :`B` 0.042729 :`A` 1.0)))

(event `self.ReceiveTick`
  (params (DeltaSeconds :type "Float (single-precision)"))
  (if (`KismetSystemLibrary.IsValid` (`self._AudioPlayer`))
    (`AudioComponent.AdjustVolume` (`self._AudioPlayer`) 0.0 (`self.Audio Volume`)))
  (if (`self.TutorialActiveBool`)
    ;[1 1 1] Tutorial
    (`|ExecutionSequence`
      (:`then_0`
        (`/Engine/EditorBlueprintResources/StandardMacros.DoOnce` false :!label _label_4
          (:`Completed`
            (set `self.ActiveTutorialPart` 0)
            (`KismetSystemLibrary.Delay` 3.0)
            (`KismetSystemLibrary.PrintText` "Welcome to the Living Tomorrow Volocopter Virtual Reality Demo. Today you will be taken on a flight throughout the City of Brussels. \n")
            (bind _returnvalue (`GameplayStatics.SpawnSound2D` "/Game/artAssets/Audio/SW_TutorialPart1.SW_TutorialPart1" 1.0 1.0 0.0 null false false))
            (set `self._AudioPlayer` _returnvalue)
            (`KismetSystemLibrary.Delay` 8.0)
            (if (`self.TutorialActiveBool`)
              (`KismetSystemLibrary.PrintText` "Let’s start with a small introduction to the controls. Hold your controllers like this, with your middle finger on the grip button and your index finger on the trigger button. Form a fist by squeezing both buttons.")
              (`AudioComponent.Stop` (`self._AudioPlayer`))
              (bind _returnvalue_2 (`GameplayStatics.SpawnSound2D` "/Game/artAssets/Audio/SW_TutorialPart2.SW_TutorialPart2" 1.0 1.0 0.0 null false false))
              (set `self._AudioPlayer` _returnvalue_2)
              (`KismetSystemLibrary.Delay` 3.0)
              (if (`self.TutorialActiveBool`)
                (`self.ForceControllersVisible`)
                (set `self.ActiveTutorialPart` 1)
                (`self.TutorialPass1`)
                (set `self.TutorialInit` true))))))
      (:`then_1`
        (if (`self.TutorialInit`)
          (switch `int` (`self.ActiveTutorialPart`)
            (:`1`
              (`self.TutorialPass1`))
            (:`2`
              (`self.ForceHandsVisible`)
              (`KismetSystemLibrary.PrintText` "Very good. \nLook around to find the camera, when you’ve spotted it, form a fist near it to grab the camera.")
              (`AudioComponent.Stop` (`self._AudioPlayer`))
              (bind _returnvalue_3 (`GameplayStatics.SpawnSound2D` "/Game/artAssets/Audio/SW_TutorialPart3.SW_TutorialPart3" 1.0 1.0 0.0 null false false))
              (set `self._AudioPlayer` _returnvalue_3)
              (set `self.ActiveTutorialPart` 3))
            (:`3`
              (`self.TutorialPass2`))
            (:`4`
              (if (`self._TutorialPass2`)
                (`KismetSystemLibrary.PrintText` "Do you see that button on the side? You can press it to take a picture. Try taking pictures of the various landmarks you’ll encounter on the trip.")
                (`AudioComponent.Stop` (`self._AudioPlayer`))
                (bind _returnvalue_4 (`GameplayStatics.SpawnSound2D` "/Game/artAssets/Audio/SW_TutorialPart4.SW_TutorialPart4" 1.0 1.0 0.0 null false false))
                (set `self._AudioPlayer` _returnvalue_4)
                (set `self.ActiveTutorialPart` 5)))
            (:`5`
              (`self.TutorialPass3`))
            (:`6`
              (if (`self._TutorialPass3`)
                (`KismetSystemLibrary.PrintText` "Put the camera to the side for now. Can you see the tablet in front of you? You can interact with it just like any other tablet, using your index finger. Point by only squeezing the grip button on your controller.")
                (`AudioComponent.Stop` (`self._AudioPlayer`))
                (bind _returnvalue_5 (`GameplayStatics.SpawnSound2D` "/Game/artAssets/Audio/SW_TutorialPart5.SW_TutorialPart5" 1.0 1.0 0.0 null false false))
                (set `self._AudioPlayer` _returnvalue_5)
                (set `self.ActiveTutorialPart` 7)))
            (:`7`
              (`KismetSystemLibrary.Delay` 12.0)
              (set `self.ActiveTutorialPart` 8))
            (:`8`
              (`KismetSystemLibrary.PrintText` "One last thing, during the flight you will be able to alter the flight route by grabbing and moving the stick. This way you will make small asjustments from the path that the auto pilot will take.")
              (`AudioComponent.Stop` (`self._AudioPlayer`))
              (bind _returnvalue_6 (`GameplayStatics.SpawnSound2D` "/Game/artAssets/Audio/SW_TutorialPart6.SW_TutorialPart6" 1.0 1.0 0.0 null false false))
              (set `self._AudioPlayer` _returnvalue_6)
              (set `self.ActiveTutorialPart` 9))
            (:`9`
              (`self.TutorialPass4`))
            (:`10`
              (`KismetSystemLibrary.PrintText` "That’s all for now. We are taking off, sit back, and enjoy the ride.")
              (`AudioComponent.Stop` (`self._AudioPlayer`))
              (bind _returnvalue_7 (`GameplayStatics.SpawnSound2D` "/Game/artAssets/Audio/SW_TutorialPart7.SW_TutorialPart7" 1.0 1.0 0.0 null false false))
              (set `self._AudioPlayer` _returnvalue_7)
              (set `self.TutorialActiveBool` false :!label _label_5)
              (`self.FadeOutStartSphere`)
              (`KismetSystemLibrary.Delay` 2.0)
              (`SceneComponent.SetVisibility` (`self.TutorialSpace`) false false)
              (bind _returnvalue_8 (`GameplayStatics.GetActorOfClass` "/Game/Blueprints/BP_Volocopter.BP_Volocopter_C"))
              (`Volocopter.SetIsVolocopterMoving` _returnvalue_8 true))))))))

(event `PPFadeToColor`
  (params (Length :type "Float (double-precision)") (Color :type "LinearColor Structure"))
  ;[1 1 1] Fade Handling
  (`TimelineComponent.SetTimelineLength` (`self.PostProcessFade`) Length)
  (`KismetMaterialLibrary.SetVectorParameterValue` "/Game/Blueprints/MPC_FadeControls.MPC_FadeControls" "FadeColor" Color)
  (bind (_direction _newtrack_0) (`Timeline|PostProcessFade` :!label _label_6)
    (:`Update`
      (`KismetMaterialLibrary.SetScalarParameterValue` "/Game/Blueprints/MPC_FadeControls.MPC_FadeControls" "FadeWeight" _newtrack_0))))

(event `PPFadeFromColor`
  (params (Length :type "Float (double-precision)") (Color :type "LinearColor Structure" :default (struct :`A` 1.0)))
  ;[1 1 1] Fade Handling
  (`TimelineComponent.SetTimelineLength` (`self.PostProcessFade`) Length)
  (`KismetMaterialLibrary.SetVectorParameterValue` "/Game/Blueprints/MPC_FadeControls.MPC_FadeControls" "FadeColor" Color)
  (goto _label_6 :!via `ReverseFromEnd`))

(event `PPTransition`
  (params (TransitionDuration :type "Float (double-precision)") (FadeLength :type "Float (double-precision)") (Color :type "LinearColor Structure"))
  ;[1 1 1] Fade Handling
  (`self.PPFadeToColor` FadeLength Color)
  (`KismetSystemLibrary.Delay` TransitionDuration)
  (`self.PPFadeFromColor` FadeLength Color))

(event `Key|Enter`
  (params (Key :type "Key Structure"))
  (bind __audioplayer (`self._AudioPlayer`))
  ;[1 1 1] Tutorial
  (:`Pressed`
    (if (`self.TutorialActiveBool`)
      (`/Engine/EditorBlueprintResources/StandardMacros.IsValid` __audioplayer
        (:`Is Valid`
          (`AudioComponent.Stop` __audioplayer))
        (:`Is Not Valid`
          _))
      (`/Engine/EditorBlueprintResources/StandardMacros.CompareInt` (`self.ActiveTutorialPart`) 1
        (:`>`
          (goto _label_5))
        (:`==`
          (`self.ForceHandsVisible`)
          (goto _label_5))
        (:`<`
          (goto _label_5))))))

(fn `ForceControllersVisible`
  (`SceneComponent.SetVisibility` (`self._pRightHandMesh`) false false)
  (`SceneComponent.SetVisibility` (`self._pLeftHandMesh`) false false)
  (`SceneComponent.SetVisibility` (`self.SM_RightController`) true false)
  (`SceneComponent.SetVisibility` (`self.SM_LeftController`) true false))

(fn `ForceHandsVisible`
  (`SceneComponent.SetVisibility` (`self._pRightHandMesh`) true false)
  (`SceneComponent.SetVisibility` (`self._pLeftHandMesh`) true false)
  (`SceneComponent.SetVisibility` (`self.SM_RightController`) false false)
  (`SceneComponent.SetVisibility` (`self.SM_LeftController`) false false))

(fn `SetControllerMaterials`
  (bind _sm_leftcontroller (`self.SM_LeftController`))
  (bind _sm_rightcontroller (`self.SM_RightController`))
  (bind _sm_rightcontroller_2 (`self.SM_RightController`))
  (bind _returnvalue (`KismetMaterialLibrary.CreateDynamicMaterialInstance` (`PrimitiveComponent.GetMaterial` _sm_rightcontroller_2 1) "RightGripMAT"))
  (bind _output_get (set `self._RightGripMAT` _returnvalue))
  (bind _returnvalue_2 (`KismetMaterialLibrary.CreateDynamicMaterialInstance` (`PrimitiveComponent.GetMaterial` _sm_rightcontroller 2) "RightTriggerMAT"))
  (bind _output_get_2 (set `self._RightTriggerMAT` _returnvalue_2))
  (bind _returnvalue_3 (`KismetMaterialLibrary.CreateDynamicMaterialInstance` (`PrimitiveComponent.GetMaterial` _sm_leftcontroller 1) "LeftTriggerMAT"))
  (bind _output_get_3 (set `self._LeftTriggerMAT` _returnvalue_3))
  (bind _returnvalue_4 (`KismetMaterialLibrary.CreateDynamicMaterialInstance` (`PrimitiveComponent.GetMaterial` _sm_leftcontroller 2) "LeftGripMAT"))
  (bind _output_get_4 (set `self._LeftGripMAT` _returnvalue_4))
  (`PrimitiveComponent.SetMaterial` _sm_rightcontroller_2 1 _output_get)
  (`PrimitiveComponent.SetMaterial` _sm_rightcontroller 2 _output_get_2)
  (`PrimitiveComponent.SetMaterial` _sm_leftcontroller 1 _output_get_3)
  (`PrimitiveComponent.SetMaterial` _sm_leftcontroller 2 _output_get_4))

(fn `ToggleVisibile`
  (`SceneComponent.ToggleVisibility` (`self._pRightHandMesh`) false)
  (`SceneComponent.ToggleVisibility` (`self._pLeftHandMesh`) false)
  (`SceneComponent.ToggleVisibility` (`self.SM_RightController`) false)
  (`SceneComponent.ToggleVisibility` (`self.SM_LeftController`) false))

(fn `TutorialPass1`
  (if (< 20.0 (`self._AudioRepeatTimer`))
    (`AudioComponent.Stop` (`self._AudioPlayer`))
    (bind _returnvalue (`GameplayStatics.SpawnSound2D` "/Game/artAssets/Audio/SW_TutorialPart2.SW_TutorialPart2" 1.0 1.0 2.8 null false false))
    (set `self._AudioPlayer` _returnvalue)
    (set `self._AudioRepeatTimer` 0.0))
  (if (`KismetMathLibrary.BooleanNOR` (and (`self._MotionControllerRTriggerHold`) (`self._MotionControllerRGripHold`)) (and (`self._MotionControllerLTriggerHold`) (`self._MotionControllerLGripHold`)))
    (`MaterialInstanceDynamic.SetScalarParameterValue` (`self._RightTriggerMAT`) "IsBlinking" 1.0)
    (`MaterialInstanceDynamic.SetScalarParameterValue` (`self._RightGripMAT`) "IsBlinking" 1.0)
    (`MaterialInstanceDynamic.SetScalarParameterValue` (`self._LeftTriggerMAT`) "IsBlinking" 1.0)
    (`MaterialInstanceDynamic.SetScalarParameterValue` (`self._LeftGripMAT`) "IsBlinking" 1.0)
    (set `self._TutorialPass1` false)
    (`VictoryBPFunctionLibrary.VictoryFloatPlusEquals` (`self._AudioRepeatTimer`) (`GameplayStatics.GetWorldDeltaSeconds`))
    (else
      (`MaterialInstanceDynamic.SetScalarParameterValue` (`self._RightTriggerMAT`) "IsBlinking" 0.0)
      (`MaterialInstanceDynamic.SetScalarParameterValue` (`self._RightGripMAT`) "IsBlinking" 0.0)
      (`MaterialInstanceDynamic.SetScalarParameterValue` (`self._LeftTriggerMAT`) "IsBlinking" 0.0)
      (`MaterialInstanceDynamic.SetScalarParameterValue` (`self._LeftGripMAT`) "IsBlinking" 0.0)
      (set `self._TutorialPass1` true)
      (set `self.ActiveTutorialPart` 2)
      (set `self._AudioRepeatTimer` 0.0))))

(fn `TutorialPass2`
  (bind __audiorepeattimer (`self._AudioRepeatTimer`))
  (`VictoryBPFunctionLibrary.VictoryFloatPlusEquals` __audiorepeattimer (`GameplayStatics.GetWorldDeltaSeconds`))
  (if (< 20.0 __audiorepeattimer)
    (`AudioComponent.Stop` (`self._AudioPlayer`))
    (bind _returnvalue (`GameplayStatics.SpawnSound2D` "/Game/artAssets/Audio/SW_TutorialPart3.SW_TutorialPart3" 1.0 1.0 1.0 null false false))
    (set `self._AudioPlayer` _returnvalue)
    (set `self._AudioRepeatTimer` 0.0))
  (cast `Polaroid` (`self._pGrabbedObject`))
  (`KismetSystemLibrary.PrintString` "PolaroidGrabbed")
  (set `self._TutorialPass2` true)
  (set `self.ActiveTutorialPart` 4)
  (set `self._AudioRepeatTimer` 0.0))

(fn `TutorialPass3`
  (bind __audiorepeattimer (`self._AudioRepeatTimer`))
  (`VictoryBPFunctionLibrary.VictoryFloatPlusEquals` __audiorepeattimer (`GameplayStatics.GetWorldDeltaSeconds`))
  (if (< 12.0 __audiorepeattimer)
    (set `self.ActiveTutorialPart` 6)
    (set `self._TutorialPass3` true)
    (set `self._AudioRepeatTimer` 0.0)))

(fn `TutorialPass4`
  (bind __audiorepeattimer (`self._AudioRepeatTimer`))
  (`VictoryBPFunctionLibrary.VictoryFloatPlusEquals` __audiorepeattimer (`GameplayStatics.GetWorldDeltaSeconds`))
  (if (< 25.0 __audiorepeattimer)
    (`AudioComponent.Stop` (`self._AudioPlayer`))
    (bind _returnvalue (`GameplayStatics.SpawnSound2D` "/Game/artAssets/Audio/SW_TutorialPart6.SW_TutorialPart6" 1.0 1.0 16.5 null false false))
    (set `self._AudioPlayer` _returnvalue)
    (set `self._AudioRepeatTimer` 0.0))
  (bind _returnvalue_2 (`GameplayStatics.GetActorOfClass` "/Game/Blueprints/BP_FlightStickTarget.BP_FlightStickTarget_C"))
  (if (> (`KismetArrayLibrary.Array_Length` (`Pickupable._Holders` _returnvalue_2)) 0)
    (set `self.ActiveTutorialPart` 10)
    (set `self._AudioRepeatTimer` 0.0)))

(fn `UserConstructionScript`
  (bind __plefthandmesh (`self._pLeftHandMesh`))
  ;[1 1 1] Mirror Left Hand
  (`SceneComponent.SetWorldScale3D` __plefthandmesh (1.0 1.0 -1.0))
  (`SceneComponent.K2_SetRelativeRotation` __plefthandmesh (struct :`Roll` 90.0) false false)
  ;[1 1 1] Attach Left Hand Index Collider to Socket
  (`SceneComponent.K2_AttachToComponent` (`self._pLeftIndexPivot`) (`self._pLeftHandMesh`) "IndexSocket" "SnapToTarget" "SnapToTarget" "KeepRelative" true)
  ;[1 1 1] Attach Right Hand Index Collider to Socket
  (`SceneComponent.K2_AttachToComponent` (`self._pRightIndexPivot`) (`self._pRightHandMesh`) "IndexSocket" "SnapToTarget" "SnapToTarget" "KeepRelative" true)
  ;[1 1 1] Disable collision on grabbers
  (`PrimitiveComponent.SetCollisionEnabled` (`self._pGrabColliderLeft`) "NoCollision")
  (`PrimitiveComponent.SetCollisionEnabled` (`self._pGrabColliderRight`) "NoCollision"))