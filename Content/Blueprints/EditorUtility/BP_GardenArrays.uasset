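; BP_GardenArrays is an editor utility Blueprint that samples random locations across a Landscape.
; Its GetBounds function loops about ten thousand times, picking a random point within the central 80% of the Landscape's actor bounds on each axis.
; Each point goes to GetTerrainLocationAtLocationWorldSpace, but the result is neither stored nor returned.
; The event graph and construction script are empty.
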(fn `GetBounds`
  (bind (_origin _boxextent) (`self.GetActorBounds` (`self.Landscape`) false))
  (bind _returnvalue (- _origin (- _boxextent (* _boxextent 0.2))))
  (bind (_returnvalue_x _returnvalue_y _returnvalue_z) (`KismetMathLibrary.BreakVector` (+ _returnvalue (* _boxextent 1.6))))
  (for _ (range 10001)
    (`/Game/Blueprints/EditorUtility/BFL_SplineCorrector.GetTerrainLocationAtLocationWorldSpace` (`KismetMathLibrary.MakeVector` (`KismetMathLibrary.RandomFloatInRange` (.x _returnvalue) _returnvalue_x) (`KismetMathLibrary.RandomFloatInRange` (.y _returnvalue) _returnvalue_y) (`KismetMathLibrary.RandomFloatInRange` (.z _returnvalue) _returnvalue_z)))))

(fn `UserConstructionScript`)