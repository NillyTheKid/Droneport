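; B_SplineWidthAdjuster is an editor utility Blueprint that sets the width of a single point on a referenced spline.
; All work runs in the Construction Script, which clamps PointID to the bounds of the spline's Points array and passes it with Width to the spline's ChangeScale function.
; An invalid spline reference is reset to None, and the event graph holds only disabled placeholder events.
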(fn `UserConstructionScript`
  (bind _spline (`self.Spline`))
  (bind _returnvalue (- (`KismetArrayLibrary.Array_Length` (`/Game/Blueprints/EditorUtility/BP_CitySpline.Points` _spline)) 1))
  (`/Engine/EditorBlueprintResources/StandardMacros.IsValid` (`self.Spline`)
    (:`Is Valid`
      (if (< (`self.PointID`) 0)
        (set `self.PointID` 0)
        (elif (> (`self.PointID`) _returnvalue)
          (set `self.PointID` _returnvalue)))
      (`/Game/Blueprints/EditorUtility/BP_CitySpline.ChangeScale` _spline (`self.PointID`) (`self.Width`)))
    (:`Is Not Valid`
      (set `self.Spline` null))))