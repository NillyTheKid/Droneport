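; Editor utility spawner that lines a spline with BP_House actors: a start piece, random middle pieces and an end piece.
; SpawnUpdateHouses clears earlier houses, converts spline length to grid units, then calls DefineMesh to place each house by its grid span.
; Houses sit perpendicular to the spline, optionally flipped, with random X/Z scale.
; The spawner destroys itself after spawning and also in its Construction Script, where DefineSpline is disconnected.
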(fn `ClearHouses`
  (bind _spawnedactors (`self.SpawnedActors`))
  (for _array_element _spawnedactors
    (`self.K2_DestroyActor` _array_element))
  (`KismetArrayLibrary.Array_Clear` _spawnedactors)
  (set `self.TotalGridUnits` 0))

(fn `DefineMesh`
  (params (ID :type Integer) (CheckLength :type Boolean :default true))
  (bind (_output_mesh _output_gridspan) (break `/Game/prototypes/PR_CityGen/DataTypes/STRUCT_House` (`|GetArrayItem` (`self.Houses`) ID)))
  (bind _returnvalue (* (+ (/ (`KismetMathLibrary.Conv_IntToDouble` _output_gridspan) 2.0) (`KismetMathLibrary.Conv_IntToDouble` (`self.TotalGridUnits`))) (`self.GridSizeInCm`)))
  (bind (_location _rotation) (`/Game/prototypes/PR_CityGen/BluePrintFunctions/BFL_CityGen.GetRotationAndLocationAtDistanceAlongSpline` (`self.Spline`) _returnvalue "World"))
  (bind _returnvalue_2 (+ (.yaw _rotation) 90.0))
  (if CheckLength
    (if (< (+ (/ _output_gridspan 2) (`self.TotalGridUnits`)) (`self.GridUnits`))
      (`KismetSystemLibrary.PrintString` (`KismetStringLibrary.Conv_DoubleToString` _returnvalue) :!label _label)
      (bind _returnvalue_3 (`|SpawnActorFromClass` "/Game/prototypes/PR_CityGen/Components/Houses/BP_House.BP_House_C" (`KismetMathLibrary.MakeTransform` _location (`KismetMathLibrary.MakeRotator` (.roll _rotation) 0.0 (select `bool` (`self.isFlipped`) :`false` _returnvalue_2 :`true` (+ _returnvalue_2 180.0))) (`KismetMathLibrary.MakeVector` (`KismetMathLibrary.RandomFloatInRange` (`self.scaleXMin`) (`self.scaleXMax`)) 1.0 (`KismetMathLibrary.RandomFloatInRange` (`self.scaleZMin`) (`self.scaleZMax`)))) "Undefined" "OverrideRootScale" null _output_mesh self (`KismetArrayLibrary.Array_Length` (`self.SpawnedActors`)) null))
      (`/Game/prototypes/PR_CityGen/Components/Houses/BP_House.MakeHouse` _returnvalue_3)
      (`KismetArrayLibrary.Array_Add` (`self.SpawnedActors`) _returnvalue_3)
      (set `self.TotalGridUnits` (+ _output_gridspan (`self.TotalGridUnits`))))
    (else
      (goto _label))))

(fn `DefineSpline`
  (bind _spline (`self.Spline`))
  (bind _splinepoints (`self.SplinePoints`))
  (`SplineComponent.SetSplinePoints` _spline _splinepoints "World" true)
  (for (_ _array_index) _splinepoints
    (`SplineComponent.SetSplinePointType` _spline _array_index "Linear" true)))

(fn `Spawn /UpdateHouses`
  (locals (RandInt :type Integer))
  (bind (_output_mesh _output_gridspan) (break `/Game/prototypes/PR_CityGen/DataTypes/STRUCT_House` (`|GetArrayItem` (`self.Houses`) (`self.endID`))))
  (`self.ClearHouses`)
  (set `self.GridUnits` (`KismetMathLibrary.FTrunc` (/ (`SplineComponent.GetSplineLength` (`self.Spline`)) (`self.GridSizeInCm`))))
  (`KismetSystemLibrary.PrintString` "Hello")
  (`self.DefineMesh` (`self.startID`))
  (bind _output_get (set `self.GridUnitsWithoutEnd` (- (`self.GridUnits`) _output_gridspan)))
  (while (<= (`self.TotalGridUnits`) _output_get)
    (bind _output_get_2 (set `local.RandInt` (`KismetMathLibrary.RandomIntegerInRange` 0 (- (`KismetArrayLibrary.Array_Length` (`self.Houses`)) 1))))
    (`self.DefineMesh` _output_get_2))
  (`self.DefineMesh` (`self.endID`) false)
  (`self.K2_DestroyActor`))

(fn `updateArray`
  (`/Game/prototypes/PR_CityGen/BluePrintFunctions/BFL_CityGen.ArrayIsValidChecker` (`self.SpawnedActors`)))

(fn `UserConstructionScript`
  (`self.K2_DestroyActor`))