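; Editor utility Blueprint that scatters roughly a thousand static mesh actors across a very large area of the level.
; SpawnMeshes loops to spawn StaticMeshActors at random X/Y positions with random yaw and pitch but no roll, then assigns each a random mesh from the StaticMesh array.
; All logic lives in that one function; the construction script and event graph are empty.
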(fn `SpawnMeshes`
  (bind _staticmesh (`self.StaticMesh`))
  (for _ (range 1001)
    (bind _returnvalue (`|SpawnActorFromClass` "/Script/Engine.StaticMeshActor" (`KismetMathLibrary.MakeTransform` (`KismetMathLibrary.MakeVector` (* (`KismetMathLibrary.RandomFloat`) 1331200.0) (* (`KismetMathLibrary.RandomFloat`) 1331200.0)) (`KismetMathLibrary.RandomRotator` false)) "Undefined" "OverrideRootScale" null null))
    (`StaticMeshComponent.SetStaticMesh` (`StaticMeshActor.StaticMeshComponent` _returnvalue) (`|GetArrayItem` _staticmesh (`KismetMathLibrary.RandomIntegerInRange` 0 (- (`KismetArrayLibrary.Array_Length` _staticmesh) 1))))))

(fn `UserConstructionScript`)