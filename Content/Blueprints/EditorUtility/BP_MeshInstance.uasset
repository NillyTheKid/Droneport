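; Editor utility actor that holds one mesh as hierarchical instances and can convert them into individual house or prop actors.
; Construction applies the static mesh and cull distances.
; MakeInstances functions spawn a BP_House or BP_Prop per instance using its component-space transform, then clear the instances.
; Rotate functions turn every instance 90 degrees either way, dirtying render state only on the last update.
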(fn `ClearInstances`
  (`InstancedStaticMeshComponent.ClearInstances` (`self.HierarchicalInstancedStaticMesh`)))

(fn `Construct`
  (bind _hierarchicalinstancedstaticmesh (`self.HierarchicalInstancedStaticMesh`))
  (`StaticMeshComponent.SetStaticMesh` _hierarchicalinstancedstaticmesh (`self.staticMesh`))
  (`InstancedStaticMeshComponent.SetCullDistances` _hierarchicalinstancedstaticmesh (`self.StartCull`) (`self.EndCull`)))

(fn `MakeInstancesHouses`
  (bind _hierarchicalinstancedstaticmesh (`self.HierarchicalInstancedStaticMesh`))
  (for _index (range (`InstancedStaticMeshComponent.GetInstanceCount` _hierarchicalinstancedstaticmesh))
    (`|SpawnActorFromClass` "/Game/prototypes/PR_CityGen/Components/Houses/BP_House.BP_House_C" (`InstancedStaticMeshComponent.GetInstanceTransform` _hierarchicalinstancedstaticmesh _index false) "Undefined" "OverrideRootScale" null (`StaticMeshComponent.StaticMesh` _hierarchicalinstancedstaticmesh) null _index null))
  (`self.ClearInstances`))

(fn `MakeInstancesProps`
  (bind _hierarchicalinstancedstaticmesh (`self.HierarchicalInstancedStaticMesh`))
  (for _index (range (`InstancedStaticMeshComponent.GetInstanceCount` _hierarchicalinstancedstaticmesh))
    (bind _returnvalue (`|SpawnActorFromClass` "/Game/Blueprints/EditorUtility/BP_Prop.BP_Prop_C" (`InstancedStaticMeshComponent.GetInstanceTransform` _hierarchicalinstancedstaticmesh _index false) "Undefined" "OverrideRootScale" null (`StaticMeshComponent.StaticMesh` _hierarchicalinstancedstaticmesh) null _index null))
    (`/Game/Blueprints/EditorUtility/BP_Prop.MakeProp` _returnvalue))
  (`self.ClearInstances`))

(fn `RotateInstance-90`
  (bind _hierarchicalinstancedstaticmesh (`self.HierarchicalInstancedStaticMesh`))
  (bind _returnvalue (- (`InstancedStaticMeshComponent.GetInstanceCount` _hierarchicalinstancedstaticmesh) 1))
  (for _index (range (+ _returnvalue 1))
    (bind _outinstancetransform (`InstancedStaticMeshComponent.GetInstanceTransform` _hierarchicalinstancedstaticmesh _index true))
    (`InstancedStaticMeshComponent.UpdateInstanceTransform` (`self.HierarchicalInstancedStaticMesh`) _index (`KismetMathLibrary.MakeTransform` (.location _outinstancetransform) (`KismetMathLibrary.ComposeRotators` (.rotation _outinstancetransform) (struct :`Yaw` -90.0)) (.scale _outinstancetransform)) true (`KismetMathLibrary.Conv_IntToBool` (`KismetMathLibrary.SelectInt` 1 0 (== _index _returnvalue))) false)))

(fn `RotateInstance90`
  (bind _hierarchicalinstancedstaticmesh (`self.HierarchicalInstancedStaticMesh`))
  (bind _returnvalue (- (`InstancedStaticMeshComponent.GetInstanceCount` _hierarchicalinstancedstaticmesh) 1))
  (for _index (range (+ _returnvalue 1))
    (bind _outinstancetransform (`InstancedStaticMeshComponent.GetInstanceTransform` _hierarchicalinstancedstaticmesh _index true))
    (`InstancedStaticMeshComponent.UpdateInstanceTransform` (`self.HierarchicalInstancedStaticMesh`) _index (`KismetMathLibrary.MakeTransform` (.location _outinstancetransform) (`KismetMathLibrary.ComposeRotators` (.rotation _outinstancetransform) (struct :`Yaw` 90.0)) (.scale _outinstancetransform)) true (`KismetMathLibrary.Conv_IntToBool` (`KismetMathLibrary.SelectInt` 1 0 (== _index _returnvalue))) false)))

(fn `UserConstructionScript`
  (`self.Construct`))