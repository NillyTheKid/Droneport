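; Editor utility Blueprint that creates two parallel copies of a referenced spline, one offset to each side.
; DuplicateSpline samples a world-space point at distance D along the right vector, positive and negative, for each point of SplineRef.
; The two point arrays each feed a spawned BP_CitySpline with a plane spline mesh and fixed width.
; The event graph and construction script are empty.
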(fn `DuplicateSpline`
  (bind _splineref (`self.SplineRef`))
  (bind _points (`/Game/Blueprints/EditorUtility/BP_CitySpline.Points` _splineref))
  (bind _spline (`/Game/Blueprints/EditorUtility/BP_CitySpline.Spline` _splineref))
  (`KismetArrayLibrary.Array_Clear` (`self.PointsRight`))
  (`KismetArrayLibrary.Array_Clear` (`self.PointsLeft`))
  (for (_ _array_index) _points
    (`KismetArrayLibrary.Array_Add` (`self.PointsLeft`) (`/Game/Blueprints/EditorUtility/BFL_SplineCorrector.GetRightPointAtDistanceAtSplinePoint` _spline _array_index (`self.d`) "World")))
  (for (_ _array_index_2) _points
    (`KismetArrayLibrary.Array_Add` (`self.PointsRight`) (`/Game/Blueprints/EditorUtility/BFL_SplineCorrector.GetRightPointAtDistanceAtSplinePoint` _spline _array_index_2 (* (`self.d`) -1.0) "World")))
  (`|SpawnActorFromClass` "/Game/Blueprints/EditorUtility/BP_CitySpline.BP_CitySpline_C" (`KismetMathLibrary.MakeTransform` (0.0 0.0 0.0)) "Undefined" "OverrideRootScale" null (`self.PointsLeft`) "/Engine/BasicShapes/Plane.Plane" 100.0 "NewEnumerator0" 0.0 0 false false false false false false false 0.0 false false false false false null)
  (`|SpawnActorFromClass` "/Game/Blueprints/EditorUtility/BP_CitySpline.BP_CitySpline_C" (`KismetMathLibrary.MakeTransform` (0.0 0.0 0.0)) "Undefined" "OverrideRootScale" null (`self.PointsRight`) "/Engine/BasicShapes/Plane.Plane" 100.0 "NewEnumerator0" 0.0 0 false false false false false false false 0.0 false false false false false null))

(fn `UserConstructionScript`)