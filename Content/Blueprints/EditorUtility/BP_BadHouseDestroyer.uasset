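; BP_BadHouseDestroyer is an editor utility actor that clears houses and props intruding on a spline-generated row.
; MoveActor places it along the parent spline at a fraction of its length, matching the spline's rotation.
; Construct sizes the box and builds an ignore list from itself and the parent spline's spawned houses, lamps, props and trees.
; DestroyOverlap runs a box overlap there, printing and destroying any other BP_House or BP_Prop found.
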(fn `Construct`
  (bind _parentspline (`self.ParentSpline`))
  (`BoxComponent.SetBoxExtent` (`self.Box`) (`self.Bounds`) true)
  (bind _output_get (set `self.ToIgnore` (`|MakeArray` self :!type "Actor Object Reference")))
  (`KismetArrayLibrary.Array_Append` _output_get (`/Game/Blueprints/EditorUtility/BP_CitySpline_Confined.SpawnedHousesLeft` _parentspline))
  (`KismetArrayLibrary.Array_Append` _output_get (`/Game/Blueprints/EditorUtility/BP_CitySpline_Confined.SpawnedHousesRight` _parentspline))
  (`KismetArrayLibrary.Array_Append` _output_get (`/Game/Blueprints/EditorUtility/BP_CitySpline_Confined.SpawnedLamps` _parentspline))
  (`KismetArrayLibrary.Array_Append` _output_get (`/Game/Blueprints/EditorUtility/BP_CitySpline_Confined.SpawnedProps` _parentspline))
  (`KismetArrayLibrary.Array_Append` _output_get (`/Game/Blueprints/EditorUtility/BP_CitySpline_Confined.SpawnedTrees` _parentspline)))

(fn `DestroyOverlap`
  (bind _box (`self.Box`))
  (bind (_outactors _returnvalue) (`KismetSystemLibrary.BoxOverlapActors` (`SceneComponent.K2_GetComponentLocation` _box) (`BoxComponent.BoxExtent` _box) (`|MakeArray` "ObjectTypeQuery2" "ObjectTypeQuery1" "ObjectTypeQuery3" :!type "EObjectTypeQuery Enum") null (`self.ToIgnore`)))
  (if _returnvalue
    (for _array_element _outactors
      (bind _asbp_house (cast `/Game/prototypes/PR_CityGen/Components/Houses/BP_House` _array_element)
        (:`then`
          (`KismetSystemLibrary.PrintString` (`KismetSystemLibrary.GetDisplayName` _asbp_house))
          (`self.K2_DestroyActor` _asbp_house))
        (:`CastFailed`
          (bind _asbp_prop (cast `/Game/Blueprints/EditorUtility/BP_Prop` _array_element))
          (`KismetSystemLibrary.PrintString` (`KismetSystemLibrary.GetDisplayName` _asbp_prop))
          (`self.K2_DestroyActor` _asbp_prop))))))

(fn `MoveActor`
  (params (D :type "Float (double-precision)"))
  (bind _spline (`/Game/Blueprints/EditorUtility/BP_CitySpline_Confined.Spline` (`self.ParentSpline`)))
  (bind _returnvalue (* (`SplineComponent.GetSplineLength` _spline) D))
  (`SceneComponent.K2_SetWorldLocationAndRotation` (`self.DefaultSceneRoot`) (`SplineComponent.GetLocationAtDistanceAlongSpline` _spline _returnvalue "World") (`SplineComponent.GetRotationAtDistanceAlongSpline` _spline _returnvalue "World") false false))

(fn `UserConstructionScript`)