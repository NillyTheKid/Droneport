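; Blueprint function library in EditorUtility with geometry helpers for splines and terrain height lookup.
; Spline helpers gather point locations, set every point's type, and offset along the right vector by point index or distance.
; A segment check keeps points within a radius and snaps others to the closest point on the line.
; Terrain helpers run vertical complex traces on one object type, falling back to zero height or the input position.
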(fn `Distance To Spline`
  (params (Point :type "Vector Structure") (SplineStart :type "Vector Structure") (SplineEnd :type "Vector Structure") (Radius :type "Float (double-precision)"))
  (returns (Distance :type "Float (double-precision)") (PointOnSpline :type "Vector Structure") (CorrectedPoint :type "Vector Structure") (IsInRadius :type Boolean))
  (bind _returnvalue (`TKMathFunctionLibrary.ClosestPointOnLineSeqment` Point SplineStart SplineEnd))
  (bind _returnvalue_2 (`KismetMathLibrary.Vector_Distance` Point _returnvalue))
  (bind _returnvalue_3 (< _returnvalue_2 Radius))
  (return _returnvalue_2 _returnvalue (`KismetMathLibrary.SelectVector` _returnvalue Point (not _returnvalue_3)) _returnvalue_3))

(fn `GetRightPointAtDistanceAtDistanceAlongSpline`
  (params (Spline :type "SplineComponent Object Reference") (DistOnSpline :type "Float (double-precision)") (Distance :type "Float (double-precision)") (CoordinateSpace :type "ESplineCoordinateSpace Enum" :default "Local"))
  (returns (Location :type "Vector Structure"))
  (return (+ (* (`SplineComponent.GetRightVectorAtDistanceAlongSpline` Spline DistOnSpline CoordinateSpace) Distance) (`SplineComponent.GetLocationAtDistanceAlongSpline` Spline DistOnSpline CoordinateSpace))))

(fn `GetRightPointAtDistanceAtSplinePoint`
  (params (Spline :type "SplineComponent Object Reference") (PointIndex :type Integer) (Distance :type "Float (double-precision)") (CoordinateSpace :type "ESplineCoordinateSpace Enum" :default "Local"))
  (returns (Location :type "Vector Structure"))
  (return (+ (* (`SplineComponent.GetRightVectorAtSplinePoint` Spline PointIndex CoordinateSpace) Distance) (`SplineComponent.GetLocationAtSplinePoint` Spline PointIndex CoordinateSpace))))

(fn `GetSplinePoints`
  (params (Spline :type "SplineComponent Object Reference") (CoordinateSpace :type "ESplineCoordinateSpace Enum" :default "Local"))
  (returns (Points :type "Array of Vector Structure"))
  (locals (PointsData :type "Array of Vector Structure"))
  (for _index (range (`SplineComponent.GetNumberOfSplinePoints` Spline))
    (`KismetArrayLibrary.Array_Add` (`local.PointsData`) (`SplineComponent.GetLocationAtSplinePoint` Spline _index CoordinateSpace)))
  (return (`local.PointsData`)))

(fn `GetTerrainLocationAtLocationWorldSpace`
  (params (InPosition :type "Vector Structure"))
  (returns (LocOut :type "Vector Structure"))
  (locals (Actors :type "Array of Actor Object Reference"))
  (bind (_outhit _returnvalue) (`KismetSystemLibrary.LineTraceSingleForObjects` :`Start` (`KismetMathLibrary.MakeVector` InPosition_X InPosition_Y -100000.0) :`End` (`KismetMathLibrary.MakeVector` InPosition_X InPosition_Y 100000.0) :`ObjectTypes` (`|MakeArray` "ObjectTypeQuery7" :!type "EObjectTypeQuery Enum") :`bTraceComplex` true :`DrawDebugType` "ForOneFrame"))
  (if _returnvalue
    (return (`.Location` (`GameplayStatics.BreakHitResult` _outhit)))
    (else
      (return (`KismetMathLibrary.MakeVector` InPosition_X InPosition_Y InPosition_Z)))))

(fn `LandScapeHeightAtLocation`
  (params (X :type "Float (double-precision)") (Y :type "Float (double-precision)"))
  (returns (Height :type "Float (double-precision)") (Location :type "Vector Structure") (ReturnValue :type Boolean))
  (bind (_outhit _returnvalue) (`KismetSystemLibrary.LineTraceSingleForObjects` :`Start` (`KismetMathLibrary.MakeVector` X Y -1000000000.0) :`End` (`KismetMathLibrary.MakeVector` X Y 1000000000.0) :`ObjectTypes` (`|MakeArray` "ObjectTypeQuery7" :!type "EObjectTypeQuery Enum") :`bTraceComplex` true :`DrawDebugType` "ForDuration"))
  (if _returnvalue
    (return (.z (`.Location` (`GameplayStatics.BreakHitResult` _outhit))) (`KismetMathLibrary.MakeVector` X Y (.z (`.Location` (`GameplayStatics.BreakHitResult` _outhit)))) _returnvalue)
    (else
      (return 0.0 (`KismetMathLibrary.MakeVector` X Y) _returnvalue))))

(fn `MakeSplineType`
  (params (Spline :type "SplineComponent Object Reference (by ref)") (Type :type "ESplinePointType Enum" :default "Linear"))
  (for _index (range (`SplineComponent.GetNumberOfSplinePoints` Spline))
    (`SplineComponent.SetSplinePointType` Spline _index Type true)))