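; City spline actor that builds a deformed mesh strip along a Points array, with road-type settings for cars, water, train and street features.
; Construction sets curved world-space points, then rebuilds one spline mesh per segment, scaled by Width and widened for cars.
; Helper functions re-apply width, rebuild with toggled collision and print segment debug data.
; SetData loads type settings from DT_RoadProperties, but its construction-script call is disconnected.
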(fn `ChangeScale`
  (params (ID :type Integer) (scale :type "Float (double-precision)" :default 1.0))
  (bind _splinemeshcomponents (`self.SplineMeshComponents`))
  (bind _output (`|GetArrayItem` _splinemeshcomponents ID))
  (if (>= ID 1)
    (`SplineMeshComponent.SetStartScale` _output (`KismetMathLibrary.MakeVector2D` scale scale) true)
    (`SplineMeshComponent.SetEndScale` (`|GetArrayItem` _splinemeshcomponents (- ID 1)) (`KismetMathLibrary.MakeVector2D` scale scale) true)
    (else
      (`SplineMeshComponent.SetStartScale` _output (`KismetMathLibrary.MakeVector2D` scale scale) true))))

(fn `ChangeWidth`
  (bind _width (`self.width`))
  (for _index (range (+ (- (`SplineComponent.GetNumberOfSplinePoints` (`self.Spline`)) 2) 1))
    (`self.ChangeScale` _index (select `bool` (`self.IsCars`) :`false` _width :`true` (+ (* _width 2.0) 1.0)))))

(fn `CreateSplineMesh`
  (params (`Collision Handling` :type "ECollisionEnabled Enum" :default "NoCollision"))
  (bind _spline (`self.Spline`))
  (bind _splinemeshcomponents (`self.SplineMeshComponents`))
  (bind _width (`self.width`))
  (bind _returnvalue (`SplineComponent.GetNumberOfSplinePoints` (`self.Spline`)))
  (bind _returnvalue_2 (- _returnvalue 2))
  (for _array_element _splinemeshcomponents
    (`ActorComponent.K2_DestroyComponent` _array_element))
  (`KismetArrayLibrary.Array_Clear` _splinemeshcomponents)
  (`KismetSystemLibrary.PrintString` (`KismetStringLibrary.Conv_IntToString` _returnvalue_2))
  (for _index (range (+ _returnvalue_2 1))
    (bind _returnvalue_3 (`AddComponent|NODE_AddSplineMeshComponent-1`))
    (`StaticMeshComponent.SetStaticMesh` _returnvalue_3 (`self.SplineMesh`))
    (`SceneComponent.K2_AttachToComponent` _returnvalue_3 (`self.DefaultSceneRoot`) "None" "KeepRelative" "KeepRelative" "KeepRelative" true)
    (`PrimitiveComponent.SetMaterial` _returnvalue_3 0 (`self.MaterialSource`))
    (bind (_location _tangent) (`SplineComponent.GetLocationAndTangentAtSplinePoint` _spline _index "World"))
    (bind (_location_2 _tangent_2) (`SplineComponent.GetLocationAndTangentAtSplinePoint` _spline (+ _index 1) "World"))
    (`SplineMeshComponent.SetStartAndEnd` _returnvalue_3 _location _tangent _location_2 (select `bool` (== _tangent_2 (0.0 0.0 0.0) :`ErrorTolerance` 0.001) :`false` _tangent_2 :`true` (1.0 1.0 0.0)) true)
    (`SplineMeshComponent.SetSplineUpDir` _returnvalue_3 (0.0 0.0 1.0) true)
    (`PrimitiveComponent.SetCollisionEnabled` _returnvalue_3 `Collision Handling`)
    (`PrimitiveComponent.SetCullDistance` _returnvalue_3 20000.0)
    (`KismetArrayLibrary.Array_Add` (`self.SplineMeshComponents`) _returnvalue_3))
  (for _index_2 (range (+ _returnvalue 1))
    (`self.ChangeScale` _index_2 (select `bool` (`self.IsCars`) :`false` _width :`true` (+ (* _width 2.0) 1.0)))))

(fn `DebugSplines`
  (for (_array_element _array_index) (`self.SplineMeshComponents`)
    (`KismetSystemLibrary.PrintString` (`KismetStringLibrary.Concat_StrStr` (`KismetStringLibrary.Conv_IntToString` _array_index) ": " (`KismetSystemLibrary.GetDisplayName` _array_element) ": " " \nEnd Position: " (`KismetStringLibrary.Conv_VectorToString` (`SplineMeshComponent.GetEndPosition` _array_element)) "| Start Position: " (`KismetStringLibrary.Conv_VectorToString` (`SplineMeshComponent.GetStartPosition` _array_element)) " \n|| Start Tangent: " (`KismetStringLibrary.Conv_VectorToString` (`SplineMeshComponent.GetStartTangent` _array_element)) "| End Tangent: " (`KismetStringLibrary.Conv_VectorToString` (`SplineMeshComponent.GetEndTangent` _array_element)) " \n|| Start Scale: " (`KismetStringLibrary.Conv_Vector2dToString` (`SplineMeshComponent.GetStartScale` _array_element)) "| End Scale: " (`KismetStringLibrary.Conv_Vector2dToString` (`SplineMeshComponent.GetEndScale` _array_element))) true true (make `LinearColor` (`KismetMathLibrary.RandomFloat`) (`KismetMathLibrary.RandomFloat`) (`KismetMathLibrary.RandomFloat`) 1.0) 10.0)))

(fn `MakeEditorMesh`
  (`self.CreateSplineMesh` "NoCollision"))

(fn `set Data`
  (bind _returnvalue (`KismetStringLibrary.Conv_StringToName` (`|GetEnumeratorNameAsString` (`self.Type`))))
  (`KismetSystemLibrary.PrintString` (`KismetStringLibrary.Conv_NameToString` _returnvalue))
  (bind _returnvalue_2 (`|GetDataTableRow` "/Game/Blueprints/STRUCT/DT_RoadProperties.DT_RoadProperties" _returnvalue)
    (:`then`
      (set `self.LaneWidth` (break `/Game/Blueprints/STRUCT/STRUCT_SplineTypeData_Test` _returnvalue_2))
      (set `self.Lanes` (`.Lanes_58_FE4C00084BD5D052702144B399F63959` (break `/Game/Blueprints/STRUCT/STRUCT_SplineTypeData_Test` _returnvalue_2)))
      (set `self.HasTrees` (`.HasTrees_59_2C71F17A4D82A0435FAD939839008764` (break `/Game/Blueprints/STRUCT/STRUCT_SplineTypeData_Test` _returnvalue_2)))
      (set `self.HasTreesRandom` (`.TreesRandom_60_684D7AAE4F627707E5B046A9015273F1` (break `/Game/Blueprints/STRUCT/STRUCT_SplineTypeData_Test` _returnvalue_2)))
      (set `self.RowTreeDistance` (`.TreesDistance_61_5F6ED9FD4FF3BED8A85245A797A4B4A9` (break `/Game/Blueprints/STRUCT/STRUCT_SplineTypeData_Test` _returnvalue_2)))
      (set `self.HasProps` (`.HasProps_62_09D536EE4C75488DBB083EA822D05CDA` (break `/Game/Blueprints/STRUCT/STRUCT_SplineTypeData_Test` _returnvalue_2)))
      (set `self.HasLights` (`.HasLights_63_DBD0E5BF4950EEA0B1A308BBBEAD5E9E` (break `/Game/Blueprints/STRUCT/STRUCT_SplineTypeData_Test` _returnvalue_2)))
      (set `self.HasHousesLeft` (`.HasHousesLeft_64_13B5899649748F3C132CF89F4590DB38` (break `/Game/Blueprints/STRUCT/STRUCT_SplineTypeData_Test` _returnvalue_2)))
      (set `self.HasHousesRight` (`.HasHousesRight_65_1EE5DF6B496C3C30CECDCEB37C82214F` (break `/Game/Blueprints/STRUCT/STRUCT_SplineTypeData_Test` _returnvalue_2)))
      (set `self.HasPedestrianZone` (`.HasPedestrianZone_66_A54398874481B4FACA3620BC1EBBC34D` (break `/Game/Blueprints/STRUCT/STRUCT_SplineTypeData_Test` _returnvalue_2)))
      (set `self.HasCyclingPath` (`.HasCyclingPath_67_39FB5E8A4F7F38CD7A365D9F38D41E21` (break `/Game/Blueprints/STRUCT/STRUCT_SplineTypeData_Test` _returnvalue_2)))
      (set `self.HasMiddles` (`.HasMiddleSeperator_68_67F80E314CA67757B6B4DFA3EE79DB2D` (break `/Game/Blueprints/STRUCT/STRUCT_SplineTypeData_Test` _returnvalue_2)))
      (set `self.IsCars` (`.IsCars_69_5CA9D25E46F25BD9FA2796821CF5872B` (break `/Game/Blueprints/STRUCT/STRUCT_SplineTypeData_Test` _returnvalue_2)))
      (set `self.IsWater` (`.IsWater_70_2CAF03CC44CACF075BE32A85B65382C0` (break `/Game/Blueprints/STRUCT/STRUCT_SplineTypeData_Test` _returnvalue_2)))
      (set `self.IsTrain` (`.IsTrain_71_E97A1EC04A378D32BAB9D9B1C035834E` (break `/Game/Blueprints/STRUCT/STRUCT_SplineTypeData_Test` _returnvalue_2))))))

(fn `ToggleCollision`
  (if (`|EnumEquality` (`PrimitiveComponent.GetCollisionEnabled` (`|GetArrayItem` (`self.SplineMeshComponents`))) "NoCollision")
    (`self.CreateSplineMesh` "QueryAndPhysics")
    (else
      (`self.CreateSplineMesh` "NoCollision"))))

(fn `UpdatePoints`
  (bind _spline (`self.Spline`))
  (`SplineComponent.SetSplinePoints` _spline (`self.Points`) "World" true)
  (for _index (range (`SplineComponent.GetNumberOfSplinePoints` _spline))
    (`SplineComponent.SetSplinePointType` (`self.Spline`) _index "Curve" true)))

(fn `UserConstructionScript`
  (bind _width (`self.width`))
  (`self.UpdatePoints`)
  (for _index (range (+ (`SplineComponent.GetNumberOfSplinePoints` (`self.Spline`)) 1))
    (`self.ChangeScale` _index (select `bool` (`self.IsCars`) :`false` _width :`true` (+ (* _width 2.0) 1.0))))
  (`self.CreateSplineMesh` "NoCollision"))