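; BP_IntersectionDestroyer is an editor utility actor that finds spline mesh components inside its Sphere component.
; The construction script calls DestroyActors, which runs a sphere overlap at the Sphere's location and radius, filtered to SplineMeshComponent and ignoring itself.
; Despite the names, it destroys nothing: it only prints the overlap result and each found component's display name.
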(fn `DestroyActors`
  (bind _sphere (`self.Sphere`))
  (bind (_outcomponents _returnvalue) (`KismetSystemLibrary.SphereOverlapComponents` (`SceneComponent.K2_GetComponentLocation` _sphere) (`SphereComponent.SphereRadius` _sphere) (`|MakeArray` "ObjectTypeQuery2" "ObjectTypeQuery1" "ObjectTypeQuery3" "ObjectTypeQuery4" "ObjectTypeQuery5" "ObjectTypeQuery6" "ObjectTypeQuery7" :!type "EObjectTypeQuery Enum") "/Script/Engine.SplineMeshComponent" (`|MakeArray` self :!type "Actor Object Reference")))
  (`KismetSystemLibrary.PrintString` (`KismetStringLibrary.Conv_BoolToString` _returnvalue))
  (for _array_element _outcomponents
    (`KismetSystemLibrary.PrintString` (`KismetSystemLibrary.GetDisplayName` _array_element))))

(fn `UserConstructionScript`
  (`self.DestroyActors`))