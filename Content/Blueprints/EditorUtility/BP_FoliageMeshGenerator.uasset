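; Editor utility actor that generates a random foliage cluster from a list of static meshes, via its MakeNewMesh function.
; MakeNewMesh destroys previously spawned components, then adds a random number of new mesh components, each recorded in SpawnedMeshes without clearing the array.
; Each gets a random mesh, yaw and interpolated scale, positioned by flattening a random unit vector onto XY and scaling it by Radius.
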(fn `MakeNewMesh`
  (bind (_returnvalue_roll _returnvalue_pitch _returnvalue_yaw) (`KismetMathLibrary.BreakRotator` (`KismetMathLibrary.RandomRotator` true)))
  (bind _meshestospawn (`self.MeshesToSpawn`))
  (for _array_element (`self.SpawnedMeshes`)
    (`ActorComponent.K2_DestroyComponent` _array_element))
  (for _ (range (+ (`KismetMathLibrary.RandomIntegerInRange` (`self.MeshCountMin`) (`self.MeshCountMax`)) 1))
    (bind _returnvalue (`AddComponent|NODE_AddStaticMeshComponent-0` :`RelativeTransform` (`KismetMathLibrary.MakeTransform` (* (* (`KismetMathLibrary.RandomUnitVector`) (1.0 1.0 0.0)) (`self.Radius`)) (`KismetMathLibrary.MakeRotator` 0.0 0.0 _returnvalue_yaw) (`KismetMathLibrary.VLerp` (`self.ScaleMin`) (`self.ScaleMax`) (`KismetMathLibrary.RandomFloat`)))))
    (`StaticMeshComponent.SetStaticMesh` _returnvalue (`|GetArrayItem` _meshestospawn (`KismetMathLibrary.RandomIntegerInRange` 0 (- (`KismetArrayLibrary.Array_Length` _meshestospawn) 1))))
    (`KismetArrayLibrary.Array_Add` (`self.SpawnedMeshes`) _returnvalue)))

(fn `UserConstructionScript`)