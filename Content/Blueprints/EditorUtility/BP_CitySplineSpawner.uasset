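; Editor utility Blueprint that spawns a confined city street along the points of its spline.
; MakeCitySpline reads the "Streets" row of DT_RoadProperties and passes its lane and feature settings, plus the world-space spline points, to a new BP_CitySpline_Confined.
; House, tree, prop and lamp offsets derive from the road's half-width.
; The spawned actor then runs Construct, ResetData and MakeAll to build itself.
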(fn `MakeCitySpline`
  (bind _returnvalue (`|GetDataTableRow` "/Game/Blueprints/STRUCT/DT_RoadProperties.DT_RoadProperties" "Streets")
    (:`then`
      (bind _returnvalue_2 (/ (* (* (`.Lanes_58_FE4C00084BD5D052702144B399F63959` (break `/Game/Blueprints/STRUCT/STRUCT_SplineTypeData_Test` _returnvalue)) (break `/Game/Blueprints/STRUCT/STRUCT_SplineTypeData_Test` _returnvalue)) 100.0) 2.0))
      (bind _returnvalue_3 (* _returnvalue_2 0.95))
      (bind _returnvalue_4 (`|SpawnActorFromClass` "/Game/Blueprints/EditorUtility/BP_CitySpline_Confined.BP_CitySpline_Confined_C" (`KismetMathLibrary.MakeTransform` (0.0 0.0 0.0)) "Undefined" "OverrideRootScale" null (`/Game/Blueprints/EditorUtility/BFL_SplineCorrector.GetSplinePoints` (`self.Spline`) "World") "/Engine/BasicShapes/Plane.Plane" 1.0 "NewEnumerator3" (break `/Game/Blueprints/STRUCT/STRUCT_SplineTypeData_Test` _returnvalue) (`.Lanes_58_FE4C00084BD5D052702144B399F63959` (break `/Game/Blueprints/STRUCT/STRUCT_SplineTypeData_Test` _returnvalue)) (`.HasProps_62_09D536EE4C75488DBB083EA822D05CDA` (break `/Game/Blueprints/STRUCT/STRUCT_SplineTypeData_Test` _returnvalue)) (`.HasLights_63_DBD0E5BF4950EEA0B1A308BBBEAD5E9E` (break `/Game/Blueprints/STRUCT/STRUCT_SplineTypeData_Test` _returnvalue)) (`.HasHousesLeft_64_13B5899649748F3C132CF89F4590DB38` (break `/Game/Blueprints/STRUCT/STRUCT_SplineTypeData_Test` _returnvalue)) (`.HasHousesRight_65_1EE5DF6B496C3C30CECDCEB37C82214F` (break `/Game/Blueprints/STRUCT/STRUCT_SplineTypeData_Test` _returnvalue)) (`.HasTrees_59_2C71F17A4D82A0435FAD939839008764` (break `/Game/Blueprints/STRUCT/STRUCT_SplineTypeData_Test` _returnvalue)) (`.TreesRandom_60_684D7AAE4F627707E5B046A9015273F1` (break `/Game/Blueprints/STRUCT/STRUCT_SplineTypeData_Test` _returnvalue)) (`.IsCars_69_5CA9D25E46F25BD9FA2796821CF5872B` (break `/Game/Blueprints/STRUCT/STRUCT_SplineTypeData_Test` _returnvalue)) (`.TreesDistance_61_5F6ED9FD4FF3BED8A85245A797A4B4A9` (break `/Game/Blueprints/STRUCT/STRUCT_SplineTypeData_Test` _returnvalue)) (`.HasPedestrianZone_66_A54398874481B4FACA3620BC1EBBC34D` (break `/Game/Blueprints/STRUCT/STRUCT_SplineTypeData_Test` _returnvalue)) (`.HasCyclingPath_67_39FB5E8A4F7F38CD7A365D9F38D41E21` (break `/Game/Blueprints/STRUCT/STRUCT_SplineTypeData_Test` _returnvalue)) (`.HasMiddleSeperator_68_67F80E314CA67757B6B4DFA3EE79DB2D` (break `/Game/Blueprints/STRUCT/STRUCT_SplineTypeData_Test` _returnvalue)) (`.IsWater_70_2CAF03CC44CACF075BE32A85B65382C0` (break `/Game/Blueprints/STRUCT/STRUCT_SplineTypeData_Test` _returnvalue)) (`.IsTrain_71_E97A1EC04A378D32BAB9D9B1C035834E` (break `/Game/Blueprints/STRUCT/STRUCT_SplineTypeData_Test` _returnvalue)) (+ _returnvalue_2 (/ 600.0 2.0)) _returnvalue_3 _returnvalue_3 (* _returnvalue_2 0.8) false null))
      (`/Game/Blueprints/EditorUtility/BP_CitySpline_Confined.Construct` _returnvalue_4)
      (`/Game/Blueprints/EditorUtility/BP_CitySpline_Confined.Reset Data` _returnvalue_4)
      (`/Game/Blueprints/EditorUtility/BP_CitySpline_Confined.MakeAll` _returnvalue_4))))

(fn `UserConstructionScript`)