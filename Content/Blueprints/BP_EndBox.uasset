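; BP_EndBox is the end-of-route trigger that finishes and resets the droneport game when the Volocopter reaches it.
; The construction script sizes the trigger box and snaps it to the end of the BP_VolocopterPath spline.
; A Volocopter overlap fires a DoOnce that ends the player's start screen, fades in the start sphere and, after a delay, resets the game mode.
; ResetEndgame re-arms the DoOnce.
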(event `Reset Endgame`
  (bind _asbp_droneport_game_mode (cast `/Game/Blueprints/BP_DroneportGameMode` (`GameplayStatics.GetGameMode`) :!pure true))
  (goto _label :!via `Reset`))

(event `self.trigger volume.OnComponentBeginOverlap`
  (params (OverlappedComponent :type "PrimitiveComponent Object Reference") (OtherActor :type "Actor Object Reference") (OtherComp :type "PrimitiveComponent Object Reference") (OtherBodyIndex :type Integer) (bFromSweep :type Boolean) (SweepResult :type "HitResult Structure (by ref)"))
  (bind _asbp_droneport_game_mode (cast `/Game/Blueprints/BP_DroneportGameMode` (`GameplayStatics.GetGameMode`) :!pure true))
  (cast `/Game/Blueprints/BP_Volocopter` OtherActor)
  (`KismetSystemLibrary.PrintString` "VolocopterEnd")
  (bind _returnvalue (`GameplayStatics.GetActorOfClass` "/Game/Blueprints/BP_Player.BP_Player_C"))
  (`/Engine/EditorBlueprintResources/StandardMacros.DoOnce` false :!label _label
    (:`Completed`
      (`/Game/Blueprints/BP_startScreen.EndTheGame` (cast `/Game/Blueprints/BP_startScreen` (`ChildActorComponent.ChildActor` (`/Game/Blueprints/BP_Player.StartScreen` _returnvalue)) :!pure true))
      (`/Game/Blueprints/BP_Player.FadeInStartSphere` _returnvalue)
      (`KismetSystemLibrary.Delay` 2.0)
      (`/Game/Blueprints/BP_DroneportGameMode.ResetGameDoOnce` _asbp_droneport_game_mode)
      (`DroneportGameMode.ResetGame` _asbp_droneport_game_mode))))

(fn `UserConstructionScript`
  (`BoxComponent.SetBoxExtent` (`self.trigger volume`) (`self.TriggerVolumeSize`) true)
  (bind _returnvalue (`GameplayStatics.GetActorOfClass` "/Game/Blueprints/BP_VolocopterPath.BP_VolocopterPath_C"))
  (bind _output_get (set `self.Path` _returnvalue))
  (bind _output_get_2 (set `self.Spline` (`VolocopterPath._pSpline` _output_get)))
  (bind (_location _rotation) (`/Game/prototypes/PR_CityGen/BluePrintFunctions/BFL_CityGen.GetRotationAndLocationAtDistanceAlongSpline` _output_get_2 (`SplineComponent.GetSplineLength` _output_get_2) "World"))
  (`SceneComponent.K2_SetWorldLocationAndRotation` (`self.trigger volume`) _location _rotation false false))