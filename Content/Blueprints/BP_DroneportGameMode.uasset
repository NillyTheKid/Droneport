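; Game mode for a VR Droneport experience with a Volocopter, which enables the HMD, then spawns and possesses the player on BeginPlay.
; StartGame repositions the player and spawns the Volocopter with its path class, a Polaroid and a flight-stick target, passing references between them.
; A DoOnce guards the start sequence until ResetGameDoOnce re-arms it.
; Tick, the construction script and SetVoloVis are empty.
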(event `self.ReceiveTick`
  (params (DeltaSeconds :type "Float (single-precision)")))

(event `StartGame`
  (bind _player (`self.Player`))
  ;[1 1 1] Spawn game objects
  (`/Engine/EditorBlueprintResources/StandardMacros.DoOnce` false :!label _label
    (:`Completed`
      (`self.K2_SetActorTransform` (`self.Player`) (`KismetMathLibrary.MakeTransform` (0.0 0.0 0.0)) false false)
      (bind _pvolocopter (`self.SpawnVolocopter` "/Game/Blueprints/BP_VolocopterPath.BP_VolocopterPath_C" "/Game/Blueprints/BP_Volocopter.BP_Volocopter_C"))
      (bind _asbp_volocopter (cast `/Game/Blueprints/BP_Volocopter` _pvolocopter))
      (bind _output_get (set `self.Volocopter` _asbp_volocopter))
      (`self.SetPlayer` _player)
      (`Volocopter.SetPlayer` _output_get _player)
      (bind _returnvalue (`|SpawnActorFromClass` "/Game/Blueprints/BP_Polaroid.BP_Polaroid_C" (`KismetMathLibrary.MakeTransform` (0.0 0.0 0.0) (struct) (0.7 0.7 0.7)) "Undefined" "OverrideRootScale" null null))
      (`self.SetPolaroid` _returnvalue)
      (`Polaroid.SetActorsForRayIgnore` _returnvalue _output_get _player (`/Game/Blueprints/BP_Player.StartScreen` _player))
      (`/Game/Blueprints/BP_Volocopter.SetPolaroidIdlePos` _output_get _returnvalue)
      (`Volocopter.DEBUG_SetPolaroid` _output_get _returnvalue)
      (bind _returnvalue_2 (`|SpawnActorFromClass` "/Game/Blueprints/BP_FlightStickTarget.BP_FlightStickTarget_C" (`KismetMathLibrary.MakeTransform` (0.0 0.0 0.0) (struct) (0.7 0.7 0.7)) "Undefined" "OverrideRootScale" null null))
      (`self.SetFlightStickTarget` _returnvalue_2)
      (`Volocopter.SetFlightStickTarget` _output_get _returnvalue_2))))

(event `self.ReceiveBeginPlay`
  ;[1 1 1] Enable VR
  (`HeadMountedDisplayFunctionLibrary.EnableHMD` true)
  (`KismetSystemLibrary.ExecuteConsoleCommand` "fullscreen" null)
  ;[1 1 1] Spawn game objects
  (bind _returnvalue (`|SpawnActorFromClass` "/Game/Blueprints/BP_Player.BP_Player_C" (`KismetMathLibrary.MakeTransform` (10000.0 10000.0 10000.0)) "Undefined" "OverrideRootScale" null null))
  (set `self.Player` _returnvalue)
  (`Controller.Possess` (`GameplayStatics.GetPlayerControllerFromID` 0) _returnvalue))

(event `ResetGameDoOnce`
  ;[1 1 1] Spawn game objects
  (goto _label :!via `Reset`))

(fn `Set Volo Vis`
  (params (Volocopter :type "/Game/Blueprints/BP_Volocopter Object Reference") (bNewVisibility :type Boolean)))

(fn `UserConstructionScript`)