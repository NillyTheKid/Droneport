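; BP_Pda is a PDA device with Home, Clock, Weather and Radio apps, plus a colour app.
; The construction script registers each named app root, assigns its button data, and links red, green and blue buttons to the colour app component.
; On BeginPlay it plays Clair de Lune from an offset, then the audio-finished callback switches to Arabesque, restarting it whenever it ends.
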(event `self.ReceiveTick`
  (params (DeltaSeconds :type "Float (single-precision)")))

(event `self.ReceiveBeginPlay`
  (bind _audio (`self.Audio`))
  (`AudioComponent.SetSound` _audio "/Game/artAssets/Audio/SW_ClairDeLuneNonCommercial.SW_ClairDeLuneNonCommercial")
  (`AudioComponent.Play` _audio 5.0)
  (add `AudioComponent.OnAudioFinished` _audio (delegate `FinishedPlaySound`)))

(event `FinishedPlaySound`
  (bind _audio (`self.Audio`))
  (`AudioComponent.SetSound` _audio "/Game/artAssets/Audio/SW_ArabesqueNonCommercial.SW_ArabesqueNonCommercial")
  (`AudioComponent.Play` _audio 1.0))

(fn `UserConstructionScript`
  (`self.RegisterApp` "Home" (`self.HomeApp`))
  (`self.SetAppButtonData` (`self.HomeButton`) "Home")
  (`self.RegisterApp` "Clock" (`self.ClockApp`))
  (`self.SetAppButtonData` (`self.ClockAppButton`) "Clock")
  (`self.RegisterApp` "Weather" (`self.WeatherApp`))
  (`self.SetAppButtonData` (`self.WeatherAppButton`) "Weather")
  (`self.RegisterApp` "Radio" (`self.RadioApp`))
  (`self.SetAppButtonData` (`self.RadioAppButton`) "Radio")
  (`self.SetColourApp` (`self.ColourAppCode`))
  (`self.RegisterColourAppButton` (`self.ColourAppCode`) (`self.RedButton`))
  (`self.RegisterColourAppButton` (`self.ColourAppCode`) (`self.GreenButton`))
  (`self.RegisterColourAppButton` (`self.ColourAppCode`) (`self.BlueButton`)))