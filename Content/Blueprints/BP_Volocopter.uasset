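; Player-carrying Volocopter for a flight over Brussels, with landmark pictures, polaroids, a PDA and an AR display.
; Construction registers the pictures and PDA; BeginPlay starts city and rotor sounds.
; Tick drives movement, player position and stick rotation, with debug axes for user flight.
; Outside the start screen, it aims an arrow from the stick at BP_FlightStickTarget and pushes flight stats into MPC_ArUi for the AR materials.
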(event `self.ReceiveBeginPlay`
  (`/Engine/EditorBlueprintResources/StandardMacros.IsValid` self
    (:`Is Valid`
      (`GameplayStatics.PlaySound2D` "/Game/artAssets/Audio/SW_CitySounds.SW_CitySounds" 1.0 1.0 0.0 null null)
      (`GameplayStatics.PlaySound2D` "/Game/artAssets/Audio/SW_Rotors.SW_Rotors" 1.0 1.0 0.0 null null)
      (set `self._pMatParamCollection` "/Game/Blueprints/MPC_ArUi.MPC_ArUi")
      (`self.SetColourApp` (`self.Pda`))
      (bind _returnvalue (`GameplayStatics.GetActorOfClass` "/Game/Blueprints/BP_Player.BP_Player_C"))
      (set `self.Player` _returnvalue)
      (`KismetSystemLibrary.Delay` 0.01)
      (set `self._IsVolocopterMoving` false)
      (`SceneComponent.K2_SetWorldLocation` (`self.Arrow`) (`SceneComponent.GetSocketLocation` (`self.FlightStick`) "Stick_Holder") false false))))

(event `SetPolaroidIdlePos`
  (params (polaroid :type "/Game/Blueprints/BP_Polaroid Object Reference"))
  (`Polaroid.SetIdlePosComp` polaroid (`self._pPolaroidIdlePosComp`))
  (`Polaroid.SetVolocopter` polaroid self))

(event `self.ReceiveTick`
  (params (DeltaSeconds :type "Float (single-precision)"))
  (bind _player (`self.Player`))
  (`KismetSystemLibrary.PrintString` (`KismetStringLibrary.Conv_BoolToString` (`self._IsVolocopterMoving`)) false false)
  (`self.UpdateUserFlightInput`)
  (`self.Move` DeltaSeconds)
  (`self.UpdateVolocopterRotation`)
  (`self.UpdatePlayerPos`)
  (`self.UpdateFlightStickRotation`)
  (`/Engine/EditorBlueprintResources/StandardMacros.IsValid` _player
    (:`Is Valid`
      (if (not (`/Game/Blueprints/BP_Player.IsInStartScreen` _player))
        (bind _returnvalue (`GameplayStatics.GetActorOfClass` "/Game/Blueprints/BP_FlightStickTarget.BP_FlightStickTarget_C"))
        (`/Engine/EditorBlueprintResources/StandardMacros.IsValid` _returnvalue
          (:`Is Valid`
            (`SceneComponent.K2_SetWorldRotation` (`self.Arrow`) (`KismetMathLibrary.FindLookAtRotation` (`SceneComponent.K2_GetComponentLocation` (`self.Arrow`)) (`SceneComponent.K2_GetComponentLocation` (`/Game/Blueprints/BP_FlightStickTarget.Box` _returnvalue))) false false)
            (bind _output_get (set `self.Rotation` (`KismetMathLibrary.ComposeRotators` (`SceneComponent.RelativeRotation` (`self.Arrow`)) (struct :`Yaw` 90.0))))
            (`KismetSystemLibrary.PrintString` (`KismetStringLibrary.Conv_RotatorToString` _output_get) false false)
            (`self.ClearUserFlightInput`)
            (`self.SetARParameters`)))))))

(event `InputAction|DEBUG_ToggleUserFlight`
  (params (Key :type "Key Structure"))
  ;[1 1 1] User Flight Controls [DEBUG]
  (:`Released`
    (`self.ToggleUserFlight`)))

(event `InputAxis|DEBUG_VoloMoveVertical`
  (params (AxisValue :type "Float (single-precision)"))
  ;[1 1 1] User Flight Controls [DEBUG]
  (`self.SetUserFlightInput` "INPUT_VERTICAL" AxisValue))

(event `InputAxis|DEBUG_VoloMoveHorizontal`
  (params (AxisValue :type "Float (single-precision)"))
  ;[1 1 1] User Flight Controls [DEBUG]
  (`self.SetUserFlightInput` "INPUT_HORIZONTAL" AxisValue))

(event `InputAxis|DEBUG_VoloCameraY`
  (params (AxisValue :type "Float (single-precision)")))

(event `InputAxis|DEBUG_VoloCameraX`
  (params (AxisValue :type "Float (single-precision)")))

(fn `SetARParameters`
  (bind (_etaminutes _etaseconds _spottedlandmarks _maxlandmarks _temperature _speed _speedmax _speedconstant _altitude _colour) (`self.GetArUiParams`))
  (`KismetMaterialLibrary.SetScalarParameterValue` "/Game/Blueprints/MPC_ArUi.MPC_ArUi" "etaMinutes" _etaminutes)
  (`KismetMaterialLibrary.SetScalarParameterValue` "/Game/Blueprints/MPC_ArUi.MPC_ArUi" "etaSeconds" _etaseconds)
  (`KismetMaterialLibrary.SetScalarParameterValue` "/Game/Blueprints/MPC_ArUi.MPC_ArUi" "spottedLandmarks" _spottedlandmarks)
  (`KismetMaterialLibrary.SetScalarParameterValue` "/Game/Blueprints/MPC_ArUi.MPC_ArUi" "maxLandmarks" _maxlandmarks)
  (`KismetMaterialLibrary.SetScalarParameterValue` "/Game/Blueprints/MPC_ArUi.MPC_ArUi" "temperature" _temperature)
  (`KismetMaterialLibrary.SetScalarParameterValue` "/Game/Blueprints/MPC_ArUi.MPC_ArUi" "speed" _speed)
  (`KismetMaterialLibrary.SetScalarParameterValue` "/Game/Blueprints/MPC_ArUi.MPC_ArUi" "speedMax" _speedmax)
  (`KismetMaterialLibrary.SetScalarParameterValue` "/Game/Blueprints/MPC_ArUi.MPC_ArUi" "altitude" _altitude)
  (`KismetMaterialLibrary.SetVectorParameterValue` "/Game/Blueprints/MPC_ArUi.MPC_ArUi" "ARColor" _colour)
  (`KismetSystemLibrary.PrintString` (`KismetStringLibrary.Concat_StrStr` (`KismetStringLibrary.Conv_DoubleToString` _etaminutes) ";" (`KismetStringLibrary.Conv_DoubleToString` _etaseconds) ";" (`KismetStringLibrary.Conv_DoubleToString` _spottedlandmarks) ";" (`KismetStringLibrary.Conv_DoubleToString` _maxlandmarks) ";" (`KismetStringLibrary.Conv_DoubleToString` _temperature) ";" (`KismetStringLibrary.Conv_DoubleToString` _speed) ";" (`KismetStringLibrary.Conv_DoubleToString` _speedmax) ";" (`KismetStringLibrary.Conv_DoubleToString` _altitude)) false false (struct :`G` 0.66 :`B` 1.0 :`A` 1.0) 0.0))

(fn `UserConstructionScript`
  (`self.RegisterPicture` (`self.Picture_BrusselNoord`) "BrusselNoord")
  (`self.RegisterPicture` (`self.Picture_Atomium`) "Atomium")
  (`self.RegisterPicture` (`self.Picture_LaekenCastle`) "LaekenCastle")
  (`self.RegisterPicture` (`self.Picture_Zaventem`) "Zaventem")
  (`self.RegisterPicture` (`self.Picture_Cathedral`) "Cathedral")
  (`self.RegisterPicture` (`self.Picture_LivingTomorrow`) "LivingTomorrow")
  (`self.RegisterPicture` (`self.Picture_GrandPlace`) "GrandPlace")
  (`self.RegisterPicture` (`self.Picture_BrusselsCentral`) "BrusselCentraal")
  (`self.RegisterPicture` (`self.Picture_Botanique`) "Botanique")
  (`self.RegisterPicture` (`self.Picture_EuropeanDistrict`) "EuropeanDistrict")
  (`self.RegisterPicture` (`self.Picture_Palace`) "Palace")
  (`self.RegisterPicture` (`self.Picture_FinanceTower`) "FinanceTower")
  (`self.RegisterPicture` (`self.Picture_WarandePark`) "WarandePark")
  (`self.RegisterPicture` (`self.Picture_MontDesArts`) "MontDesArts")
  (`self.RegisterPicture` (`self.Picture_Parliament`) "Parliament")
  (`self.SetPda` (`self.Pda`)))