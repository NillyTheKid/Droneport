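; Start screen actor that fades its screen mesh and sphere out when the game starts and back in when it ends.
; Both meshes get dynamic materials on BeginPlay, with Opacity driven by one timeline and the sphere delayed by Timeoffset.
; StartTheGame plays the timeline forward and EndTheGame reverses it, using cross-reset DoOnce gates against retriggering.
; The construction script sets playback rate from Tutorialspeed.
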(event `InitMat`
  (bind _startscreen (`self.startScreen`))
  (bind _sphere (`self.Sphere`))
  (bind _returnvalue (`KismetMaterialLibrary.CreateDynamicMaterialInstance` (`PrimitiveComponent.GetMaterial` _sphere 0)))
  (bind _output_get (set `self.sphere_mat` _returnvalue))
  (`PrimitiveComponent.SetMaterial` _sphere 0 _output_get)
  (bind _returnvalue_2 (`KismetMaterialLibrary.CreateDynamicMaterialInstance` (`PrimitiveComponent.GetMaterial` _startscreen 0)))
  (bind _output_get_2 (set `self.Screen_mat` _returnvalue_2))
  (`PrimitiveComponent.SetMaterial` _startscreen 0 _output_get_2)
  (`KismetSystemLibrary.PrintString` "Startscreen Mat Init" true true (struct :`R` 1.0 :`G` 0.922414 :`A` 1.0)))

(event `self.ReceiveBeginPlay`
  (`self.InitMat`))

(event `StartTheGame`
  (`|ExecutionSequence`
    (:`then_0`
      (`/Engine/EditorBlueprintResources/StandardMacros.DoOnce` false :!label _label
        (:`Completed`
          (bind (_direction _float_track) (`Timeline|Timeline_0` :!via `PlayFromStart` :!label _label_2)
            (:`Update`
              (`MaterialInstanceDynamic.SetScalarParameterValue` (`self.Screen_mat`) "Opacity" (`KismetMathLibrary.Lerp` 1.0 0.0 (`KismetMathLibrary.FClamp` _float_track)))
              (`MaterialInstanceDynamic.SetScalarParameterValue` (`self.sphere_mat`) "Opacity" (`KismetMathLibrary.Lerp` 1.0 0.0 (`KismetMathLibrary.FClamp` (- _float_track (`self.timeoffset`))))))))))
    (:`then_1`
      (goto _label_3 :!via `Reset`))))

(event `EndTheGame`
  (`SceneComponent.SetVisibility` (`self.DefaultSceneRoot`) true false)
  (`|ExecutionSequence`
    (:`then_0`
      (`/Engine/EditorBlueprintResources/StandardMacros.DoOnce` false :!label _label_3
        (:`Completed`
          (goto _label_2 :!via `ReverseFromEnd`))))
    (:`then_1`
      (goto _label :!via `Reset`))))

(fn `UserConstructionScript`
  (`TimelineComponent.SetPlayRate` (`self.Timeline_0`) (`self.tutorialspeed`)))