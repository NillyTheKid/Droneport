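; Spline-placed trigger that teleports along the volocopter path behind a black screen fade.
; The construction script finds the BP_VolocopterPath, places the trigger box at StartDistance on its spline and a cube at the destination, TeleportTargetDistance further along.
; When BP_Volocopter first overlaps, the player's post-process fades to black, the path's Teleport runs with TeleportTargetDistance, then the view fades back in.
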(event `self.trigger volume.OnComponentBeginOverlap`
  (params (OverlappedComponent :type "PrimitiveComponent Object Reference") (OtherActor :type "Actor Object Reference") (OtherComp :type "PrimitiveComponent Object Reference") (OtherBodyIndex :type Integer) (bFromSweep :type Boolean) (SweepResult :type "HitResult Structure (by ref)"))
  (cast `/Game/Blueprints/BP_Volocopter` OtherActor)
  (bind _returnvalue (`GameplayStatics.GetActorOfClass` "/Game/Blueprints/BP_Player.BP_Player_C"))
  (`/Engine/EditorBlueprintResources/StandardMacros.DoOnce` false
    (:`Completed`
      (`/Game/Blueprints/BP_Player.PPFadeToColor` :`self` _returnvalue :`Length` 2.0)
      (`KismetSystemLibrary.Delay` 2.0)
      (`/Game/Blueprints/BP_VolocopterPath.Teleport` (`self.Path`) (`self.TeleportTargetDistance`))
      (`KismetSystemLibrary.Delay` 0.5)
      (`/Game/Blueprints/BP_Player.PPFadeFromColor` _returnvalue 2.0 (struct :`A` 1.0)))))

(fn `UserConstructionScript`
  (bind _startdistance (`self.StartDistance`))
  (`BoxComponent.SetBoxExtent` (`self.trigger volume`) (`self.TriggerVolumeSize`) true)
  (bind _returnvalue (`GameplayStatics.GetActorOfClass` "/Game/Blueprints/BP_VolocopterPath.BP_VolocopterPath_C"))
  (bind _output_get (set `self.Path` _returnvalue))
  (bind _output_get_2 (set `self.Spline` (`VolocopterPath._pSpline` _output_get)))
  (bind (_location _rotation) (`/Game/prototypes/PR_CityGen/BluePrintFunctions/BFL_CityGen.GetRotationAndLocationAtDistanceAlongSpline` _output_get_2 (+ _startdistance (`self.TeleportTargetDistance`)) "World"))
  (`SceneComponent.K2_SetWorldLocationAndRotation` (`self.Cube`) _location _rotation false false)
  (bind (_location_2 _rotation_2) (`/Game/prototypes/PR_CityGen/BluePrintFunctions/BFL_CityGen.GetRotationAndLocationAtDistanceAlongSpline` _output_get_2 _startdistance "World"))
  (`SceneComponent.K2_SetWorldLocationAndRotation` (`self.trigger volume`) _location_2 _rotation_2 false false))