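; BP_Polaroid is a Polaroid camera that takes pictures, built on a parent class that supplies the capture, positioning and button logic.
; Construction passes the box collider and view plane to the parent, and Tick updates the position.
; Button collider overlaps or the F key run the press handler, playing a shutter-location sound when it succeeds; overlap end releases.
; Successful captures play a 2D sound, and a debug input takes pictures directly.
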(event `self.ReceiveTick`
  (params (DeltaSeconds :type "Float (single-precision)"))
  (`self.UpdatePosition`))

(event `Key|F`
  (params (Key :type "Key Structure"))
  (:`Pressed`
    ;[1 1 1] Handle Button being pressed
    (bind _isfinger (`self.HandleButtonCollisionEnter` (stale `self._pButtonCollider.OnComponentBeginOverlap` OtherComp) :!label _label))
    (if _isfinger
      (`GameplayStatics.PlaySoundAtLocation` "/Game/artAssets/Audio/SW_Polaroid.SW_Polaroid" (`self.K2_GetActorLocation`) (struct) 1.0 1.0 0.0 null null null))))

(event `self._pButtonCollider.OnComponentBeginOverlap`
  (params (OverlappedComponent :type "PrimitiveComponent Object Reference") (OtherActor :type "Actor Object Reference") (OtherComp :type "PrimitiveComponent Object Reference") (OtherBodyIndex :type Integer) (bFromSweep :type Boolean) (SweepResult :type "HitResult Structure (by ref)"))
  ;[1 1 1] Handle Button being pressed
  (goto _label))

(event `self._pButtonCollider.OnComponentEndOverlap`
  (params (OverlappedComponent :type "PrimitiveComponent Object Reference") (OtherActor :type "Actor Object Reference") (OtherComp :type "PrimitiveComponent Object Reference") (OtherBodyIndex :type Integer))
  ;[1 1 1] Handle Button being pressed
  (`self.HandleButtonCollisionExit` OtherComp))

(event `InputAction|DEBUG_TakePicture`
  (params (Key :type "Key Structure"))
  (:`Pressed`
    (`self.TakePicture`)))

(fn `OnSuccesfulImageTaken`
  (returns (imageTransform :type "Transform Structure"))
  (bind _imagetransform (`parent.OnSuccesfulImageTaken`))
  (`GameplayStatics.SpawnSound2D` "/Game/artAssets/Audio/SW_PolaroidSucces.SW_PolaroidSucces" 1.0 1.0 0.0 null)
  (return _imagetransform))

(fn `UserConstructionScript`
  (`self.SetColliderComp` (`self._pBoxCollider`))
  (`self.SetViewPlane` (`self.ViewPlane`)))