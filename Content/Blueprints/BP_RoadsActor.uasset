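; Road actor that builds a flat strip along its Points in the construction script, using its Mat material and Width.
; Construct destroys the previous spline meshes, then AddSplineMesh creates a world-space spline and one Plane spline mesh per segment.
; Segments have no collision, a cull distance and a fallback for zero end tangents.
; A second pass scales segment ends to Width, with debug prints left in.
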(fn `AddSplineMesh`
  (params (Points :type "Array of Vector Structure") (Material :type "MaterialInstance Object Reference") (Width :type "Float (double-precision)"))
  (bind _splinemesh (`self.SplineMesh`))
  (bind _returnvalue (`AddComponent|NODE_AddSplineComponent-0`))
  (`SplineComponent.SetSplinePoints` _returnvalue Points "World" true)
  (bind _returnvalue_2 (`SplineComponent.GetNumberOfSplinePoints` _returnvalue))
  (bind _returnvalue_3 (- _returnvalue_2 2))
  (`KismetSystemLibrary.PrintString` (`KismetStringLibrary.Conv_IntToString` _returnvalue_3))
  (for _index (range (+ _returnvalue_3 1))
    (bind _returnvalue_4 (`AddComponent|NODE_AddSplineMeshComponent-1`))
    (`StaticMeshComponent.SetStaticMesh` _returnvalue_4 "/Engine/BasicShapes/Plane.Plane")
    (`SceneComponent.K2_AttachToComponent` _returnvalue_4 null "None" "KeepWorld" "KeepWorld" "KeepWorld" true)
    (`PrimitiveComponent.SetMaterial` _returnvalue_4 0 Material)
    (bind (_location _tangent) (`SplineComponent.GetLocationAndTangentAtSplinePoint` _returnvalue _index "World"))
    (bind (_location_2 _tangent_2) (`SplineComponent.GetLocationAndTangentAtSplinePoint` _returnvalue (+ _index 1) "World"))
    (`SplineMeshComponent.SetStartAndEnd` _returnvalue_4 _location _tangent _location_2 (select `bool` (== _tangent_2 (0.0 0.0 0.0) :`ErrorTolerance` 0.001) :`false` _tangent_2 :`true` (1.0 1.0 0.0)) true)
    (`SplineMeshComponent.SetSplineUpDir` _returnvalue_4 (0.0 0.0 1.0) true)
    (`PrimitiveComponent.SetCollisionEnabled` _returnvalue_4 "NoCollision")
    (`PrimitiveComponent.SetCullDistance` _returnvalue_4 250000.0)
    (`KismetArrayLibrary.Array_Add` (`self.SplineMesh`) _returnvalue_4))
  (for _index_2 (range _returnvalue_2)
    (`KismetSystemLibrary.PrintString` "Hello")
    (if (>= _index_2 1)
      (bind _output (`|GetArrayItem` _splinemesh _index_2))
      (`SplineMeshComponent.SetStartScale` _output (`KismetMathLibrary.MakeVector2D` Width Width) true)
      (`SplineMeshComponent.SetEndScale` (`|GetArrayItem` _splinemesh (- _index_2 1)) (`KismetMathLibrary.MakeVector2D` Width Width) true)
      (else
        (`SplineMeshComponent.SetStartScale` _output (`KismetMathLibrary.MakeVector2D` Width Width) true)))))

(fn `Construct`
  (bind _splinemesh (`self.SplineMesh`))
  (for _array_element _splinemesh
    (`/Engine/EditorBlueprintResources/StandardMacros.IsValid` _array_element
      (:`Is Valid`
        (`ActorComponent.K2_DestroyComponent` _array_element))))
  (`KismetArrayLibrary.Array_Clear` _splinemesh)
  (`self.AddSplineMesh` (`self.Points`) (`self.Mat`) (`self.Width`)))

(fn `UserConstructionScript`
  (`self.Construct`))