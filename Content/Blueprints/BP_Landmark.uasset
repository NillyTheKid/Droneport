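; BP_Landmark is a landmark actor that builds static meshes from a list and carries a billboard plane.
; Construction adds the meshes, moves the plane and a cube to the billboard location, and feeds name ID, minimum distance and plane position into a dynamic billboard material.
; Tick resets the plane's world rotation to zero every frame.
; An Overlap function returns props and houses overlapping its collider.
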(event `self.ReceiveTick`
  (params (DeltaSeconds :type "Float (single-precision)"))
  (`SceneComponent.K2_SetWorldRotation` :`self` (`self.Plane`)))

(fn `MakeMesh`
  (for _array_element (`self._pMeshes`)
    (bind _returnvalue (`AddComponent|NODE_AddStaticMeshComponent-0`))
    (`StaticMeshComponent.SetStaticMesh` _returnvalue _array_element)))

(fn `Overlap`
  (returns (Props :type "Array of Actor Object Reference"))
  (locals (NewLocalVar_0 :type "Array of Actor Object Reference"))
  (bind __pcollidercomponent (`self._pColliderComponent`))
  (bind _output_get (set `local.NewLocalVar_0` (`PrimitiveComponent.GetOverlappingActors` __pcollidercomponent "/Game/Blueprints/EditorUtility/BP_Prop.BP_Prop_C")))
  (`KismetArrayLibrary.Array_Append` _output_get (`PrimitiveComponent.GetOverlappingActors` __pcollidercomponent "/Game/prototypes/PR_CityGen/Components/Houses/BP_House.BP_House_C"))
  (return _output_get))

(fn `UserConstructionScript`
  (bind _plane (`self.Plane`))
  (bind _billboardlocation (`self.BillboardLocation`))
  (`self.MakeMesh`)
  (`SceneComponent.K2_SetRelativeLocation` _plane _billboardlocation false false)
  (`SceneComponent.K2_SetRelativeLocation` (`self.Cube`) _billboardlocation false false)
  (bind _returnvalue (`KismetMaterialLibrary.CreateDynamicMaterialInstance` "/Game/artAssets/_common/Shaders/MI_Billboard.MI_Billboard"))
  (bind _output_get (set `self.Mat` _returnvalue))
  (`MaterialInstanceDynamic.SetScalarParameterValue` _output_get "ID" (`KismetMathLibrary.Conv_IntToDouble` (`self.NameID`)))
  (`MaterialInstanceDynamic.SetScalarParameterValue` _output_get "DistanceMin" (`self.Minimum Dist`))
  (`MaterialInstanceDynamic.SetVectorParameterValue` _output_get "BillboardPosition" (`KismetMathLibrary.Conv_VectorToLinearColor` (`SceneComponent.K2_GetComponentLocation` _plane)))
  (`PrimitiveComponent.SetMaterial` _plane 0 _output_get))