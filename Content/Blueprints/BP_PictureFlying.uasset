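; Picture actor that slides a plane out of a Polaroid, then floats it along a wandering spline toward an arrow marker.
; A curved source spline from the picture exit to the arrow is resampled into a path, whose points get random offsets weighted by a cosine-power falloff strongest mid-path.
; While UpdatePoints is set, Tick rebuilds and re-randomizes the path; the slide timeline's finish clears it and starts the float timeline.
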(event `self.ReceiveTick`
  (params (DeltaSeconds :type "Float (single-precision)"))
  (if (`self.UpdatePoints`)
    (`self.DrawBaseSpline`)
    (`self.DrawSampleSpline`)
    (`self.RandomizeSample`)))

(event `self.ReceiveBeginPlay`
  (bind _splinepath (`self.SplinePath`))
  (bind _polaroid (`self.Polaroid`))
  (bind _picturesource (`/Game/Blueprints/BP_Polaroid.PictureSource` _polaroid))
  (bind _pictureend (`/Game/Blueprints/BP_Polaroid.PictureEnd` _polaroid))
  (`self.DrawBaseSpline`)
  (`self.DrawSampleSpline`)
  (`self.RandomizeSample`)
  (`TimelineComponent.SetTimelineLength` (`self.Slidetime_`) (`self.SlideTime`))
  (`TimelineComponent.SetTimelineLength` (`self.FloatyTime`) (`self.FloatTime`))
  (bind (_direction _slidetime) (`Timeline|Slidetime_` :!via `PlayFromStart`)
    (:`Update`
      (`SceneComponent.K2_SetWorldTransform` (`self.Plane`) (`KismetMathLibrary.MakeTransform` (`KismetMathLibrary.VLerp` (`SceneComponent.K2_GetComponentLocation` _picturesource) (`SceneComponent.K2_GetComponentLocation` _pictureend) _slidetime) (`KismetMathLibrary.RLerp` (`SceneComponent.K2_GetComponentRotation` _picturesource) (`SceneComponent.K2_GetComponentRotation` _pictureend) _slidetime) (0.15 0.15 0.15)) false false))
    (:`Finished`
      (set `self.UpdatePoints` false)
      (bind (_direction_2 _floatytime) (`Timeline|FloatyTime` :!via `PlayFromStart`)
        (:`Update`
          (bind _returnvalue (* _floatytime (`SplineComponent.GetSplineLength` (`self.SplinePath`))))
          (`SceneComponent.K2_SetWorldTransform` (`self.Plane`) (`KismetMathLibrary.MakeTransform` (`SplineComponent.GetLocationAtDistanceAlongSpline` _splinepath _returnvalue "World") (`SplineComponent.GetRotationAtDistanceAlongSpline` _splinepath _returnvalue "World") (0.15 0.15 0.15)) false false))))))

(fn `Distribution`
  (params (U :type "Float (double-precision)") (CurveSlope :type "Float (double-precision)"))
  (returns (Weight :type "Float (double-precision)"))
  (return (`KismetMathLibrary.MultiplyMultiply_FloatFloat` (`KismetMathLibrary.Cos` (/ (* U 3.141593) 2.0)) CurveSlope)))

(fn `DrawBaseSpline`
  (bind _arrow (`self.Arrow`))
  (bind _splinesource (`self.SplineSource`))
  (bind _returnvalue (`SceneComponent.K2_GetComponentLocation` _arrow))
  (bind _pictureend (`/Game/Blueprints/BP_Polaroid.PictureEnd` (`self.Polaroid`)))
  (bind _returnvalue_2 (`SceneComponent.K2_GetComponentLocation` _pictureend))
  (bind _returnvalue_3 (* (`KismetMathLibrary.Vector_Distance` _returnvalue_2 _returnvalue) 3.1415))
  (`SplineComponent.SetSplinePoints` _splinesource (`|MakeArray` _returnvalue_2 _returnvalue) "World" true)
  (`SplineComponent.SetTangentAtSplinePoint` _splinesource 0 (* (`SceneComponent.GetForwardVector` _pictureend) _returnvalue_3) "World" true)
  (`SplineComponent.SetTangentAtSplinePoint` _splinesource 1 (* (* (`SceneComponent.GetForwardVector` _arrow) -1.0) _returnvalue_3) "World" true))

(fn `DrawSampleSpline`
  (bind _returnvalue (- (`self.PointCount`) 1))
  (`KismetArrayLibrary.Array_Clear` (`self.Points`))
  (`KismetArrayLibrary.Array_Clear` (`self.Points`))
  (for _index (range (+ _returnvalue 1))
    (bind _location (`self.SampleSourceSpline` _index _returnvalue "Local" "World"))
    (`KismetArrayLibrary.Array_Add` (`self.Points`) _location))
  (`SplineComponent.SetSplinePoints` (`self.SplinePath`) (`self.Points`) "Local" true))

(fn `InitialSlide`)

(fn `RandomizeSample`
  (for (_ _array_index) (`/Game/Blueprints/EditorUtility/BFL_SplineCorrector.GetSplinePoints` (`self.SplinePath`))
    (bind _offset (`self.RandomOffset` _array_index (`self.RandomOffsetRadius`) (`self.Distribution` (`KismetMathLibrary.Lerp` -0.99 0.99 (/ (`KismetMathLibrary.Conv_IntToDouble` _array_index) (`KismetMathLibrary.Conv_IntToDouble` (- (`self.PointCount`) 1)))) 3.5)))
    (`SplineComponent.SetLocationAtSplinePoint` (`self.SplinePath`) _array_index _offset "World" true)))

(fn `RandomOffset`
  (params (ID :type Integer) (Radius :type "Float (double-precision)") (DistortionWeight :type "Float (double-precision)"))
  (returns (Offset :type "Vector Structure"))
  (bind _splinepath (`self.SplinePath`))
  (return (+ (* (+ (+ (* (`KismetMathLibrary.Normal` (`SplineComponent.GetRightVectorAtSplinePoint` _splinepath ID "World")) (`KismetMathLibrary.RandomFloatInRange` Radius (* Radius -1.0))) (* (`KismetMathLibrary.Normal` (`SplineComponent.GetUpVectorAtSplinePoint` _splinepath ID "World")) (`KismetMathLibrary.RandomFloatInRange` Radius (* Radius -1.0)))) (* (`KismetMathLibrary.Normal` (`SplineComponent.GetTangentAtSplinePoint` _splinepath ID "World")) (`KismetMathLibrary.RandomFloatInRange` Radius (* Radius -1.0)))) DistortionWeight) (`SplineComponent.GetLocationAtSplinePoint` _splinepath ID "World"))))

(fn `SampleSourceSpline`
  (params (CurrentIndex :type Integer) (MaxIndex :type Integer) (LocationCoordinateSpace :type "ESplineCoordinateSpace Enum" :default "Local") (TangentCoordinateSpace :type "ESplineCoordinateSpace Enum" :default "Local"))
  (returns (Location :type "Vector Structure") (Tangent :type "Vector Structure"))
  (bind _splinesource (`self.SplineSource`))
  (bind _returnvalue (* (/ (`KismetMathLibrary.Conv_IntToDouble` CurrentIndex) (`KismetMathLibrary.Conv_IntToDouble` MaxIndex)) (`SplineComponent.GetSplineLength` _splinesource)))
  (return (`SplineComponent.GetLocationAtDistanceAlongSpline` _splinesource _returnvalue LocationCoordinateSpace) (`SplineComponent.GetTangentAtDistanceAlongSpline` _splinesource _returnvalue TangentCoordinateSpace)))

(fn `UserConstructionScript`
  (`self.DrawBaseSpline`)
  (`self.DrawSampleSpline`)
  (`self.RandomizeSample`))