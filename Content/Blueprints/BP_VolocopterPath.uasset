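; Spline path actor, named for a Volocopter, that drives position updates and teleports and can show or hide its route.
; BeginPlay caches the spline length and destroys existing spline mesh components.
; Tick calls UpdatePosition with zero, and Teleport forwards a distance to HandleTeleport; neither function is defined here.
; TogglePath destroys the segment meshes or rebuilds them at runtime, one spline mesh between each pair of neighboring points.
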(event `self.ReceiveTick`
  (params (DeltaSeconds :type "Float (single-precision)"))
  (`self.UpdatePosition` 0.0))

(event `self.ReceiveBeginPlay`
  ;[1 1 1] Set _SplineLength at start
  (set `self._SplineLength` (`SplineComponent.GetSplineLength` (`self._pSpline`)))
  (for _array_element (`self.SplineMesh`)
    (`/Engine/EditorBlueprintResources/StandardMacros.IsValid` _array_element
      (:`Is Valid`
        (`ActorComponent.K2_DestroyComponent` _array_element)))))

(event `Teleport`
  (params (teleportDistance :type "Float (double-precision)"))
  ;[1 1 1] Teleport
  (`self.HandleTeleport` teleportDistance))

(fn `TogglePath`
  (bind __pspline (`self._pSpline`))
  (if (`self.HasPath`)
    (for _array_element (`self.SplineMesh`) :!label _label
      (`ActorComponent.K2_DestroyComponent` _array_element))
    (set `self.HasPath` false)
    (else
      (`|ExecutionSequence`
        (:`then_0`
          (goto _label))
        (:`then_1`
          (for _index (range (+ (- (`SplineComponent.GetNumberOfSplinePoints` __pspline) 2) 1))
            (bind _returnvalue (`AddComponent|NODE_AddSplineMeshComponent-0`))
            (`SceneComponent.K2_AttachToComponent` _returnvalue (`self.RootComponent`) "None" "KeepRelative" "KeepRelative" "KeepRelative" true)
            (bind (_location _tangent) (`SplineComponent.GetLocationAndTangentAtSplinePoint` __pspline _index "World"))
            (bind (_location_2 _tangent_2) (`SplineComponent.GetLocationAndTangentAtSplinePoint` __pspline (+ _index 1) "World"))
            (`SplineMeshComponent.SetStartAndEnd` _returnvalue _location _tangent _location_2 _tangent_2 true)
            (`KismetArrayLibrary.Array_Add` (`self.SplineMesh`) _returnvalue))
          (set `self.HasPath` true))))))

(fn `UserConstructionScript`)