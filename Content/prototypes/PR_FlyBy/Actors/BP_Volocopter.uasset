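; Player-ridden volocopter for the fly-by prototype, following an externally supplied spline position and rotation past Brussels landmarks.
; Each tick, flight stick input moves the craft within a clamped offset from the spline and eases the mesh into a sideways lean.
; It rotates a seat point from look inputs, then snaps the player and stick origin to their mount points.
; Collected landmark IDs reveal matching polaroids through a map built at construction.
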(event `self.ReceiveTick`
  (params (DeltaSeconds :type "Float (single-precision)"))
  ;[1 1 1] Update loop
  (`self.GetStickControls`)
  (`self.Update Spline Offset` DeltaSeconds)
  (`self.Update Volocopter Path`)
  (`self.HandleRotation` DeltaSeconds)
  (`self.HandleLean` DeltaSeconds)
  (`self.SetCameraTransform`))

(event `self.ReceiveBeginPlay`
  (`/Engine/EditorBlueprintResources/StandardMacros.NegateFloat` (`self._ForwardRot`)))

(event `SetPlayer`
  (params (player :type "Pawn Object Reference"))
  (set `self._Player` player))

(event `SetFlightStick`
  (params (stick :type "/Game/prototypes/PR_FlyBy/Actors/BP_FlightStick Object Reference"))
  (set `self._FlightStick` stick))

(event `SetSplinePosAndRot`
  (params (Pos :type "Vector Structure") (Rot :type "Rotator Structure"))
  ;[1 1 1] SetSplinePosAndRot
  (set `self._PosOnSpline` Pos)
  (set `self._RotOnSpline` Rot))

(event `SetCameraTransform`
  (bind _flightstickpos (`self.flightStickPos`))
  ;[1 1 1] Set camera transform
  (`SceneComponent.K2_SetWorldTransform` (`Actor.RootComponent` (`self._Player`)) (`SceneComponent.K2_GetComponentToWorld` (`self.PlayerPos`)) false true)
  (`/Game/prototypes/PR_FlyBy/Actors/BP_FlightStick.SetOrigin` (`self._FlightStick`) (`SceneComponent.K2_GetComponentLocation` _flightstickpos) (`SceneComponent.K2_GetComponentRotation` _flightstickpos)))

(event `HandleCollected`
  (params (LandmarkId :type String))
  (bind (_value _returnvalue) (`BlueprintMapLibrary.Map_Find` (`self._PolaroidMap`) LandmarkId))
  ;[1 1 1] Handle collected
  (if _returnvalue
    (`SceneComponent.SetVisibility` _value true false)))

(event `Update Spline Offset`
  (params (elapsed :type "Float (double-precision)"))
  (bind _maxdistfromspline (`self.MaxDistFromSpline`))
  (bind _maxdistfromspline_2 (`self.MaxDistFromSpline`))
  (bind _returnvalue (* elapsed (`self._MoveSpeed`)))
  ;[1 1 1] Update spline offset
  (set `self._YPos` (`KismetMathLibrary.FClamp` (+ (`self._YPos`) (* _returnvalue (`self._RightInput`))) (- 0.0 _maxdistfromspline) _maxdistfromspline))
  (set `self._ZPos` (`KismetMathLibrary.FClamp` (+ (* _returnvalue (`self._UpInput`)) (`self._ZPos`)) (- 0.0 _maxdistfromspline_2) _maxdistfromspline_2)))

(event `Update Volocopter Path`
  (bind _staticmesh (`self.StaticMesh`))
  ;[1 1 1] Update copter path
  (`self.K2_SetActorLocationAndRotation` (+ (`self._PosOnSpline`) (+ (* (`SceneComponent.GetRightVector` _staticmesh) (`self._YPos`)) (* (`SceneComponent.GetUpVector` _staticmesh) (`self._ZPos`)))) (`self._RotOnSpline`)))

(event `HandleRotation`
  (params (elapsedSec :type "Float (double-precision)"))
  (bind _playerpos (`self.PlayerPos`))
  (bind _returnvalue (* elapsedSec (`self._CamRotSpeed`)))
  ;[1 1 1] Handle rotation
  (`SceneComponent.K2_AddWorldRotation` _playerpos (`KismetMathLibrary.MakeRotator` 0.0 0.0 (* _returnvalue (`self._ZRotation`))) false false)
  (`SceneComponent.K2_AddLocalRotation` _playerpos (`KismetMathLibrary.MakeRotator` 0.0 (* (`self._XRotation`) _returnvalue)) false false))

(event `GetStickControls`
  (bind __controls (`/Game/prototypes/PR_FlyBy/Actors/BP_FlightStick._Controls` (`self._FlightStick`)))
  ;[1 1 1] Get stick controls
  (if (> (`KismetMathLibrary.VSize` __controls) 0.0)
    (set `self._RightInput` (.y __controls))
    (set `self._UpInput` (.z __controls))))

(event `HandleLean`
  (params (elapsed :type "Float (double-precision)"))
  ;[1 1 1] Handle Lean
  (bind _output_get (set `self._CurrSideRot` (`self.AdjustRotation(Float)` (`self._CurrSideRot`) (* (`self._RightInput`) (`self._SideRotMax`)) (* elapsed (`self._SideRotSpeed`)))))
  (`SceneComponent.K2_SetRelativeRotation` (`self.StaticMesh`) (`KismetMathLibrary.MakeRotator` _output_get (`self._ForwardRot`)) false false))

(fn `UserConstructionScript`
  (bind __polaroidmap (`self._PolaroidMap`))
  ;[1 1 1] Set up polaroids
  (`BlueprintMapLibrary.Map_Add` __polaroidmap "Atomium" (`self.AtomiumPolaroid`))
  (`BlueprintMapLibrary.Map_Add` __polaroidmap "BrusselCentraal" (`self.BrusselCPolaroid`))
  (`BlueprintMapLibrary.Map_Add` __polaroidmap "EuropeanDistrict" (`self.EuroDistrictPolaroid`))
  (`BlueprintMapLibrary.Map_Add` __polaroidmap "BrusselNoord" (`self.BrusselNPolaroid`))
  (`BlueprintMapLibrary.Map_Add` __polaroidmap "Port" (`self.PortPolaroid`))
  (`BlueprintMapLibrary.Map_Add` __polaroidmap "Cathedral" (`self.CathedralPolaroid`))
  (`BlueprintMapLibrary.Map_Add` __polaroidmap "FinanceTower" (`self.FinanceTowerPolaroid`))
  (`BlueprintMapLibrary.Map_Add` __polaroidmap "Botanique" (`self.BotaniquePolaroid`))
  (`BlueprintMapLibrary.Map_Add` __polaroidmap "Stadium" (`self.StadiumPolaroid`))
  (`BlueprintMapLibrary.Map_Add` __polaroidmap "EuropeanParliament" (`self.EuroParlPolaroid`))
  (`BlueprintMapLibrary.Map_Add` __polaroidmap "GrandPlace" (`self.GrandPlacePolaroid`))
  (`BlueprintMapLibrary.Map_Add` __polaroidmap "Castle" (`self.CastlePolaroid`))
  (`BlueprintMapLibrary.Map_Add` __polaroidmap "MontDesArts" (`self.MontDesArtsPolaroid`))
  (`BlueprintMapLibrary.Map_Add` __polaroidmap "Palace" (`self.PalacePolaroid`))
  (`BlueprintMapLibrary.Map_Add` __polaroidmap "WarandePark" (`self.WarandeParkPolaroid`))
  (`BlueprintMapLibrary.Map_Add` __polaroidmap "Zaventem" (`self.ZaventemPolaroid`)))