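; VR motion-controller pawn for the FlyBy prototype that grips a volocopter's flight stick and photographs landmarks with a Polaroid camera.
; Holding right trigger as the hand sphere overlaps the stick grabs it, and Tick feeds it the hand position until release.
; Left trigger raycasts from the camera; landmark hits animate a photo, then report its ID to the Volocopter.
; The same ray sizes an aiming spline, and a material parameter drives screen fade.
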(event `self.Sphere.OnComponentBeginOverlap`
  (params (OverlappedComponent :type "PrimitiveComponent Object Reference") (OtherActor :type "Actor Object Reference") (OtherComp :type "PrimitiveComponent Object Reference") (OtherBodyIndex :type Integer) (bFromSweep :type Boolean) (SweepResult :type "HitResult Structure (by ref)"))
  ;[1 1 1] Grab stick
  (if (and (`self.ActorHasTag` OtherActor "FlightStick") (`self._RTriggerIsHeld`))
    (bind _asbp_flight_stick (cast `/Game/prototypes/PR_FlyBy/Actors/BP_FlightStick` OtherActor))
    (set `self._Stick` _asbp_flight_stick)))

(event `Key|MotionController_Left_Trigger`
  (params (Key :type "Key Structure"))
  (:`Pressed`
    ;[1 1 1] Raycast
    (if (`self._CanTakePicture`)
      (bind (_out_hit _return_value) (`self.Cast Camera Ray`))
      (bind (_bblockinghit _binitialoverlap _time _distance _location _impactpoint _normal _impactnormal _physmat _hitactor) (`GameplayStatics.BreakHitResult` _out_hit))
      (if (and _return_value (`self.ActorHasTag` _hitactor "Landmark"))
        (set `self._CanTakePicture` false)
        (bind _asbp_landmark_base (cast `/Game/prototypes/PR_FlyBy/Actors/BP_LandmarkBase` _hitactor))
        (bind (_direction _polaroidpos) (`Timeline|PolaroidTimeLine` :!via `PlayFromStart`)
          (:`Update`
            (`SceneComponent.K2_SetRelativeLocation` (`self.Polaroid`) _polaroidpos false false))
          (:`Finished`
            ;;[1 1 1] Collect polaroid
            (`/Game/prototypes/PR_FlyBy/Actors/BP_Volocopter.HandleCollected` (`self._Volocopter`) (`/Game/prototypes/PR_FlyBy/Actors/BP_LandmarkBase._LandmarkId` _asbp_landmark_base))
            (set `self._CanTakePicture` true)
            (`SceneComponent.K2_SetRelativeLocation` (`self.Polaroid`) (0.0 0.0 0.0) false false)))))))

(event `Key|MotionController_Right_Trigger`
  (params (Key :type "Key Structure"))
  ;[1 1 1] Right hand controls
  (:`Pressed`
    (`MaterialInstanceDynamic.SetVectorParameterValue` (`self._RHandMat`) "Colour" (struct :`R` 0.044785 :`G` 1.0 :`A` 1.0))
    (set `self._RTriggerIsHeld` true))
  (:`Released`
    (`MaterialInstanceDynamic.SetVectorParameterValue` (`self._RHandMat`) "Colour" (struct :`R` 1.0 :`G` 1.0 :`B` 1.0 :`A` 1.0))
    (set `self._RTriggerIsHeld` false)
    (if (`KismetSystemLibrary.IsValid` (`self._Stick`))
      (set `self._Stick` null))))

(event `SetVolocopter`
  (params (volocopter :type "/Game/prototypes/PR_FlyBy/Actors/BP_Volocopter Object Reference"))
  ;[1 1 1] Set volocopter
  (set `self._Volocopter` volocopter))

(event `self.ReceiveTick`
  (params (DeltaSeconds :type "Float (single-precision)"))
  ;[1 1 1] Update loop
  (`self.Update HandPos`)
  (`self.Update Aiming Spline`))

(event `SetFadeOpacity`
  (params (opacity :type "Float (double-precision)"))
  (`MaterialInstanceDynamic.SetScalarParameterValue` (`self._FadeMat`) "Opacity" opacity))

(event `Update HandPos`
  (bind __stick (`self._Stick`))
  ;[1 1 1] Update HandPos
  (if (`KismetSystemLibrary.IsValid` __stick)
    (`/Game/prototypes/PR_FlyBy/Actors/BP_FlightStick.SetHandPos` __stick (`SceneComponent.K2_GetComponentLocation` (`self.Sphere`)))))

(event `Update Aiming Spline`
  ;[1 1 1] Update aiming spline
  (`SplineMeshComponent.SetSplineUpDir` (`self.Aiming Spline`) (- (`SceneComponent.K2_GetComponentLocation` (`self.Camera`)) (`SceneComponent.K2_GetComponentLocation` (`self.PolaroidCam`))) true)
  (bind _out_hit (`self.Cast Camera Ray`))
  (bind (_bblockinghit _binitialoverlap _time _distance) (`GameplayStatics.BreakHitResult` _out_hit))
  (`SplineMeshComponent.SetEndPosition` (`self.Aiming Spline`) (`KismetMathLibrary.MakeVector` (select `bool` _bblockinghit :`false` (`self._RayLength`) :`true` _distance)) true))

(fn `Cast Camera Ray`
  (returns (`out hit` :type "HitResult Structure") (`return value` :type Boolean))
  (bind _polaroidcam (`self.PolaroidCam`))
  (bind _returnvalue (`SceneComponent.K2_GetComponentLocation` _polaroidcam))
  (bind (_outhit _returnvalue_2) (`KismetSystemLibrary.LineTraceSingle` _returnvalue (+ _returnvalue (* (`SceneComponent.GetForwardVector` _polaroidcam) (`self._RayLength`))) "TraceTypeQuery1" false (`|MakeArray` (`self._Volocopter`) :!type "Actor Object Reference") "None" true (struct :`R` 1.0 :`A` 1.0) (struct :`G` 1.0 :`A` 1.0) 3.0))
  (return _outhit _returnvalue_2))

(fn `UserConstructionScript`
  (bind _returnvalue (`PrimitiveComponent.CreateDynamicMaterialInstance` (`self.Sphere`) 0 "/Game/PR_VrInteractivtyTest/M_SolidColour.M_SolidColour" "None"))
  (set `self._RHandMat` _returnvalue)
  (bind _returnvalue_2 (`PrimitiveComponent.CreateDynamicMaterialInstance` (`self.Sphere1`) 0 "/Game/prototypes/PR_FlyBy/Mat/M_FadeMat.M_FadeMat" "None"))
  (set `self._FadeMat` _returnvalue_2))