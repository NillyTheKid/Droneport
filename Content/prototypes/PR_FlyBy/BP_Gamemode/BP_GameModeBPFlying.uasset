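; Game mode for the FlyBy flying prototype that assembles the flight setup at BeginPlay.
; It spawns a flyby pawn, a Volocopter and a flight stick at the origin, giving the Volocopter references to the pawn and stick.
; The pawn and an existing spline visualizer in the level receive the Volocopter reference.
; Player controller 0 then possesses the pawn, not the Volocopter.
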(event `self.ReceiveBeginPlay`
  (bind _returnvalue (`KismetMathLibrary.MakeTransform` (0.0 0.0 0.0)))
  ;[1 1 1] Initialize
  (bind _returnvalue_2 (`|SpawnActorFromClass` "/Game/prototypes/PR_FlyBy/Actors/BP_FlybyPawn.BP_FlybyPawn_C" _returnvalue "Undefined" "OverrideRootScale" null null))
  (bind _returnvalue_3 (`|SpawnActorFromClass` "/Game/prototypes/PR_FlyBy/Actors/BP_Volocopter.BP_Volocopter_C" _returnvalue "Undefined" "OverrideRootScale" null null))
  (`/Game/prototypes/PR_FlyBy/Actors/BP_Volocopter.SetPlayer` _returnvalue_3 _returnvalue_2)
  (bind _returnvalue_4 (`|SpawnActorFromClass` "/Game/prototypes/PR_FlyBy/Actors/BP_FlightStick.BP_FlightStick_C" _returnvalue "Undefined" "OverrideRootScale" null null))
  (`/Game/prototypes/PR_FlyBy/Actors/BP_Volocopter.SetFlightStick` _returnvalue_3 _returnvalue_4)
  (bind _returnvalue_5 (`GameplayStatics.GetActorOfClass` "/Game/prototypes/PR_FlyBy/Actors/BP_SplineVisualizer.BP_SplineVisualizer_C"))
  (`/Game/prototypes/PR_FlyBy/Actors/BP_SplineVisualizer.SetVolocopter` _returnvalue_5 _returnvalue_3)
  (`/Game/prototypes/PR_FlyBy/Actors/BP_FlybyPawn.SetVolocopter` _returnvalue_2 _returnvalue_3)
  (`Controller.Possess` (`GameplayStatics.GetPlayerControllerFromID` 0) _returnvalue_2))

(fn `UserConstructionScript`)