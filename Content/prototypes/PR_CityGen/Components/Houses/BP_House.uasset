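; House actor for the city generation prototype, tied to a parent BP_BuildingSpline that tracks it in a SpawnedActors array.
; MakeHouse applies the stored Mesh to its static mesh component and prints the parent's display name.
; DeleteActor removes its stored Index from the parent's array, passes that array to ArrayIsValidChecker, then destroys the house.
; Event graph and construction script have no active logic.
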(fn `DeleteActor`
  (bind _spawnedactors (`/Game/prototypes/PR_CityGen/Components/Houses/BP_BuildingSpline.SpawnedActors` (cast `/Game/prototypes/PR_CityGen/Components/Houses/BP_BuildingSpline` (`self.ParentActor`) :!pure true)))
  (`KismetArrayLibrary.Array_Remove` _spawnedactors (`self.Index`))
  (`/Game/prototypes/PR_CityGen/BluePrintFunctions/BFL_CityGen.ArrayIsValidChecker` _spawnedactors)
  (`self.K2_DestroyActor`))

(fn `MakeHouse`
  (`KismetSystemLibrary.PrintString` (`KismetSystemLibrary.GetDisplayName` (`self.ParentActor`)))
  (`StaticMeshComponent.SetStaticMesh` (`self.StaticMesh`) (`self.Mesh`)))

(fn `UserConstructionScript`)