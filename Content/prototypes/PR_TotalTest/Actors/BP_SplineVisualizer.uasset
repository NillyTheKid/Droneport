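; Spline path actor that drives a Volocopter, handed in through SetVolocopter, along its Spline in the TotalTest prototype.
; Each Tick advances a distance counter by Speed without delta-time scaling, so movement is frame-rate dependent, and prints it on screen.
; It sends the Volocopter the world location at that distance, lowered by a fixed Z offset, and only the spline's yaw, keeping it level.
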(event `SetVolocopter`
  (params (volocopter :type "/Game/prototypes/PR_FlyBy/Actors/BP_Volocopter Object Reference"))
  (set `self.Volo` volocopter))

(event `self.ReceiveTick`
  (params (DeltaSeconds :type "Float (single-precision)"))
  (bind _counter (`self.counter`))
  (bind (_returnvalue_x _returnvalue_y _returnvalue_z) (`KismetMathLibrary.BreakVector` (`SplineComponent.GetLocationAtDistanceAlongSpline` (`self.Spline`) _counter "World")))
  (bind (_returnvalue_roll _returnvalue_pitch _returnvalue_yaw) (`KismetMathLibrary.BreakRotator` (`SplineComponent.GetRotationAtDistanceAlongSpline` (`self.Spline`) _counter "World")))
  (bind _output_get (set `self.counter` (+ (`self.counter`) (`self.speed`))))
  (`KismetSystemLibrary.PrintString` (`KismetStringLibrary.Conv_DoubleToString` _output_get) true true (struct :`R` 1.0 :`B` 0.265008 :`A` 1.0) 0.0)
  (`/Game/prototypes/PR_FlyBy/Actors/BP_Volocopter.SetSplinePosAndRot` (`self.Volo`) (`KismetMathLibrary.MakeVector` _returnvalue_x _returnvalue_y (- _returnvalue_z 750.0)) (`KismetMathLibrary.MakeRotator` 0.0 0.0 _returnvalue_yaw)))

(fn `UserConstructionScript`)