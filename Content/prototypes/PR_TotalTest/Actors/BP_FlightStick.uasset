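; BP_FlightStick is a prototype flight stick actor that turns a supplied hand position into a control vector.
; SetOrigin stores the rest point and rotation, and SetHandPos moves the stick toward the hand, clamped to MaxMovement from that origin.
; The clamped world-space offset divided by MaxMovement becomes Controls.
; A per-frame flag lets Tick snap the stick back to its origin and zero Controls when hand updates stop.
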(event `SetOrigin`
  (params (origin :type "Vector Structure") (rotation :type "Rotator Structure"))
  (set `self._Origin` origin)
  (`self.K2_SetActorRotation` rotation))

(event `SetHandPos`
  (params (`Hand position` :type "Vector Structure"))
  (`self.UpdateStickPos` `Hand position`)
  (set `self._GotHandPos` true))

(event `self.ReceiveTick`
  (params (DeltaSeconds :type "Float (single-precision)"))
  (if (not (`self._GotHandPos`))
    (set `self._HandPos` (0.0 0.0 0.0))
    (set `self._Controls` (0.0 0.0 0.0))
    (`self.K2_SetActorLocation` (`self._Origin`)))
  (set `self._GotHandPos` false))

(fn `UpdateStickPos`
  (params (`hand pos` :type "Vector Structure"))
  (locals (dist :type "Float (double-precision)") (handVector :type "Vector Structure"))
  (bind __maxmovement (`self._MaxMovement`))
  (bind __origin (`self._Origin`))
  (bind _output_get (set `self._HandPos` `hand pos`))
  (bind _output_get_2 (set `local.dist` (`KismetMathLibrary.Vector_Distance` _output_get __origin)))
  (bind _returnvalue (* (`KismetMathLibrary.Normal` (- _output_get __origin)) (`KismetMathLibrary.FClamp` _output_get_2 (- 0.0 __maxmovement) __maxmovement)))
  (set `self._Controls` (/ _returnvalue (`self._MaxMovement`)))
  (`self.K2_SetActorLocation` (+ (`self._Origin`) _returnvalue)))

(fn `UserConstructionScript`)