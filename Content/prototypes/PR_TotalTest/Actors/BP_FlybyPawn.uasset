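; BP_FlybyPawn is a prototype VR pawn for steering a Volocopter and photographing landmarks.
; Holding the right trigger tints the hand sphere; overlapping a FlightStick meanwhile grabs it, feeding it the sphere's position each tick until release.
; The left trigger line traces from the polaroid camera, ignoring the Volocopter, and passes any hit landmark's ID to the Volocopter as collected.
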(event `self.Sphere.OnComponentBeginOverlap`
  (params (OverlappedComponent :type "PrimitiveComponent Object Reference") (OtherActor :type "Actor Object Reference") (OtherComp :type "PrimitiveComponent Object Reference") (OtherBodyIndex :type Integer) (bFromSweep :type Boolean) (SweepResult :type "HitResult Structure (by ref)"))
  ;[1 1 1] Grab stick
  (if (and (`self.ActorHasTag` OtherActor "FlightStick") (`self._RTriggerIsHeld`))
    (bind _asbp_flight_stick (cast `/Game/prototypes/PR_FlyBy/Actors/BP_FlightStick` OtherActor))
    (set `self._Stick` _asbp_flight_stick)))

(event `Key|MotionController_Left_Trigger`
  (params (Key :type "Key Structure"))
  (bind _polaroidcam (`self.PolaroidCam`))
  (bind _returnvalue (`SceneComponent.K2_GetComponentLocation` _polaroidcam))
  (:`Pressed`
    ;[1 1 1] Raycast
    (bind (_outhit _returnvalue_2) (`KismetSystemLibrary.LineTraceSingle` _returnvalue (+ _returnvalue (* (`SceneComponent.GetForwardVector` _polaroidcam) (`self._RayLength`))) "TraceTypeQuery1" false (`|MakeArray` (`self._Volocopter`) :!type "Actor Object Reference") "ForDuration" true (struct :`R` 1.0 :`A` 1.0) (struct :`G` 1.0 :`A` 1.0) 3.0))
    (bind (_bblockinghit _binitialoverlap _time _distance _location _impactpoint _normal _impactnormal _physmat _hitactor) (`GameplayStatics.BreakHitResult` _outhit))
    (if (and _returnvalue_2 (`self.ActorHasTag` _hitactor "Landmark"))
      (bind _asbp_landmark_base (cast `/Game/prototypes/PR_FlyBy/Actors/BP_LandmarkBase` _hitactor))
      ;[1 1 1] Collect polaroid
      (`/Game/prototypes/PR_FlyBy/Actors/BP_Volocopter.HandleCollected` (`self._Volocopter`) (`/Game/prototypes/PR_FlyBy/Actors/BP_LandmarkBase._LandmarkId` _asbp_landmark_base)))))

(event `self.ReceiveTick`
  (params (DeltaSeconds :type "Float (single-precision)"))
  (bind __stick (`self._Stick`))
  (if (`KismetSystemLibrary.IsValid` __stick)
    (`/Game/prototypes/PR_FlyBy/Actors/BP_FlightStick.SetHandPos` __stick (`SceneComponent.K2_GetComponentLocation` (`self.Sphere`)))))

(event `Key|MotionController_Right_Trigger`
  (params (Key :type "Key Structure"))
  (:`Pressed`
    (`MaterialInstanceDynamic.SetVectorParameterValue` (`self._RHandMat`) "Colour" (struct :`R` 0.044785 :`G` 1.0 :`A` 1.0))
    (set `self._RTriggerIsHeld` true))
  (:`Released`
    (`MaterialInstanceDynamic.SetVectorParameterValue` (`self._RHandMat`) "Colour" (struct :`R` 1.0 :`G` 1.0 :`B` 1.0 :`A` 1.0))
    (set `self._RTriggerIsHeld` false)
    (if (`KismetSystemLibrary.IsValid` (`self._Stick`))
      (set `self._Stick` null))))

(event `SetVolocopter`
  (params (volocopter :type "/Game/prototypes/PR_FlyBy/Actors/BP_Volocopter Object Reference"))
  (set `self._Volocopter` volocopter))

(fn `UserConstructionScript`
  (bind _returnvalue (`PrimitiveComponent.CreateDynamicMaterialInstance` (`self.Sphere`) 0 "/Game/prototypes/PR_VrInteractivtyTest/M_SolidColour.M_SolidColour" "None"))
  (set `self._RHandMat` _returnvalue))